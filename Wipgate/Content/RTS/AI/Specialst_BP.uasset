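; Specialist unit Blueprint for the RTS that gives the unit active, construct and passive abilities.
; On BeginPlay, after the parent logic, it spawns one actor from each of the three ability classes at its own transform and stores the references.
; It then sets itself as the caster on each ability, while its construction script only calls the parent.
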(event EventBeginPlay
  (bind _returnvalue (Transformation|GetActorTransform))
  ;[1 1 1] Instantiate abilities
  (|CallParentFunction)
  (bind _returnvalue_2 (Game|SpawnActorfromClass (Variables|Default|GetAbilityActiveClass) _returnvalue "Undefined" 0 0))
  (Variables|Default|SetAbilityActive _returnvalue_2)
  (bind _returnvalue_3 (Game|SpawnActorfromClass (Variables|Default|GetAbilityConstructClass) _returnvalue "Undefined" 0 0))
  (Variables|Default|SetAbilityConstruct _returnvalue_3)
  (bind _returnvalue_4 (Game|SpawnActorfromClass (Variables|Default|GetAbilityPassiveClass) _returnvalue "Undefined" 0 0))
  (Variables|Default|SetAbilityPassive _returnvalue_4)
  ;[1 1 1] Set ability caster variable to this unit
  (bind _output_get (Variables|/Script/Wipgate.Ability|Setm_Caster (Variables|Default|GetAbilityActive) self))
  (bind _output_get_2 (Variables|/Script/Wipgate.Ability|Setm_Caster (Variables|Default|GetAbilityConstruct) _output_get))
  (Variables|/Script/Wipgate.Ability|Setm_Caster (Variables|Default|GetAbilityPassive) _output_get_2))

(fn ConstructionScript
  (|CallParentFunction))