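; FlockManager is an RTS AI manager actor that spawns a group of units and pushes a shared move target to them.
; BeginPlay scatters the units within spawn bounds, tracks them locally and registers them in the game state's entity list.
; On a timed interval, Tick copies ClickedTarget to each unit when HasTarget is set, without computing steering or setting that target itself.
; Debug spheres show centre of mass, avoidance ranges and the target.
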(event EventBeginPlay
  (bind _spawnboundsstart (Variables|Default|GetSpawnBoundsStart))
  (bind _spawnboundsend (Variables|Default|GetSpawnBoundsEnd))
  (Utilities|Casting|CastToRTS_PlayerController_BP (Game|GetPlayerController 0))
  (Input|EnableInput (Game|GetPlayerController 0))
  (for _index (range 0 (- (Variables|Default|GetNumberOfUnits) 1))
    (bind _returnvalue (Game|SpawnActorfromClass "/Game/RTS/AI/Unit.Unit_C" (Math|Conversions|ToTransform(Vector) (Math|Vector|MakeVector (Math|Random|RandomFloatinRange (.x _spawnboundsstart) (.x _spawnboundsend)) (Math|Random|RandomFloatinRange (.y _spawnboundsstart) (.y _spawnboundsend)) 1e+02)) "AdjustIfPossibleButDontSpawnIfColliding" 0 0))
    (Utilities|IsValid _returnvalue
      (:Is%20Valid
        (if true
          (Utilities|Array|Add (Variables|Default|GetUnits) _returnvalue)
          (Variables|/Script/Wipgate.RTS_Unit|SetFinalTarget _returnvalue (Math|Vector|MakeVector 0.0 0.0 0.0))
          (bind _asrts_game_state (Utilities|Casting|CastToRTS_GameState (Game|GetGameState)))
          (Utilities|Array|Add (Variables|/Script/Wipgate.RTS_GameState|GetEntities _asrts_game_state) _returnvalue))))))

(event EventTick
  (params (DeltaSeconds :type Float%20%28single-precision%29))
  (Variables|Default|SetCurrentTimer (+ DeltaSeconds (Variables|Default|GetCurrentTimer)))
  (if (>= (Variables|Default|GetCurrentTimer) (Variables|Default|GetMaxTimer))
    (Variables|Default|SetCurrentTimer 0.0)
    (if (Variables|Default|GetHasTarget)
      (for _array_element (Variables|Default|GetUnits)
        (bind _output_get (Variables|/Script/Wipgate.RTS_Unit|SetOriginalTarget _array_element (Variables|Default|GetClickedTarget)))
        (Variables|/Script/Wipgate.RTS_Unit|SetFinalTarget _array_element _output_get))
      (CallFunction|DrawDebugging))
    (else
      (CallFunction|DrawDebugging))))

(fn ConstructionScript)

(fn DrawDebugging
  (Rendering|Debug|DrawDebugSphere (Variables|Default|GetCentreOfMass) 1e+01 12 "(R=1.000000,G=0.863573,B=0.000000,A=1.000000)" 0.0 1.0)
  (for _array_element (Variables|Default|GetUnits)
    (Rendering|Debug|DrawDebugSphere (Transformation|GetActorLocation _array_element) (Variables|Default|GetUnitAvoidRange) 12 "(R=0.000000,G=0.034290,B=1.000000,A=1.000000)" 0.0 1.0))
  (Rendering|Debug|DrawDebugSphere (Variables|Default|GetClickedTarget) 1e+02 12 "(R=0.000000,G=1.000000,B=0.992820,A=1.000000)" 0.0 1.0))