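; Test area-of-effect ability for the RTS, targeted with a circle decal under the mouse cursor.
; BeginPlay attaches the decal hidden, and Tick moves the root to the cursor's world-static hit while the ability is selected.
; Activate sphere-overlaps Unit_Character pawns at that point, spawns a hit emitter on each and hides the decal.
; It only prints hit results and plays effects, applying no damage.
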(event EventBeginPlay
  ;[1 1 1] Create decal
  (bind _returnvalue (Class|GameplayStatics|SpawnDecalAttached "/Game/RTS/Blueprints/AblityTests/M_CircleDecal.M_CircleDecal" "300.000000,300.000000,300.000000" (Variables|Default|GetDefaultSceneRoot) "None" "0, 0,100.000000" "90.000000, 0, 0" "KeepRelativeOffset" 0.0))
  (Variables|Default|SetDecal1 _returnvalue)
  (CallFunction|SetDecalEnabled false)
  (Rendering|SetVisibility (Variables|Default|GetDefaultSceneRoot) false true))

(event EventTick
  (params (DeltaSeconds :type Float%20%28single-precision%29))
  ;[1 1 1] Display and move decal
  (if (Utilities|Enum|Equal(Enum) (Variables|Default|Getm_State) "E_SELECTED")
    (Transformation|SetWorldLocation (Variables|Default|GetDefaultSceneRoot) (+ (.Location (Collision|BreakHitResult (.HitResult (Class|PlayerController|GetHitResultUnderCursorforObjects (Game|GetPlayerController 0) (Utilities|Array|MakeArray "ObjectTypeQuery1") true)))) "0, 0,10.000000") false false)))

(event EventActivate
  ;[1 1 1] Ability activate
  (bind (_outactors _returnvalue) (Collision|SphereOverlapActors (Transformation|GetWorldLocation (Variables|Default|GetDefaultSceneRoot)) 3e+02 (Utilities|Array|MakeArray "ObjectTypeQuery3") "/Game/RTS/Blueprints/Unit_Character.Unit_Character_C"))
  (if _returnvalue
    (Development|PrintString "Actor hit" true false)
    (for _array_element _outactors
      (Effects|SpawnEmitteratLocation "/Game/Art/ParticleEffects/PE_Hit.PE_Hit" (Transformation|GetActorLocation _array_element))
      (CallFunction|SetDecalEnabled false))
    (else
      (Development|PrintString "No Actor Hit" true false))))

(fn ConstructionScript)

(fn SetDecalEnabled
  (params (enabled :type Boolean))
  (Rendering|SetVisibility (Variables|Default|GetDecal1) enabled false))