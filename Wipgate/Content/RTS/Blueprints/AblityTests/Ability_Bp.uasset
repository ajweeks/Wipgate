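; Base Blueprint for an RTS ability that handles targeting feedback and applies stat effects to units.
; Selecting changes the cursor; ground-targeted types hide it and show a circle decal, spawned on BeginPlay, that Tick moves to the mouse's ground position.
; Helper functions apply a timed unit effect to a single target or to units in a sphere overlap, or spawn an AreaOfEffect actor at the ability's location.
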(event EventBeginPlay
  ;[1 1 1] Create decal
  (CallFunction|InitializeDecal 3e+02))

(event EventDeselect
  ;[1 1 1] Cursor and decal handling on deselection
  (if (Utilities|Enum|Equal(Enum) (Variables|Default|Getm_State) "E_SELECTED")
    (Variables|Default|Setm_State "E_AVAILABLE")
    (Variables|/Script/Engine.PlayerController|SetCurrentMouseCursor (Game|GetPlayerController 0) "Default")
    (Class|WidgetBlueprintLibrary|SetFocustoGameViewport)
    (if (Utilities|Enum|Equal(Enum) (Variables|Default|Getm_Type) "E_TARGET_GROUND")
      (CallFunction|SetDecalEnabled false))))

(event EventTick
  (params (DeltaSeconds :type Float%20%28single-precision%29))
  ;[1 1 1] Move decal
  (if (Utilities|Enum|Equal(Enum) (Variables|Default|Getm_State) "E_SELECTED")
    (if (Utilities|Enum|Equal(Enum) (Variables|Default|Getm_Type) "E_TARGET_GROUND")
      (bind _newparam (CallFunction|GetMousePosGround))
      (Transformation|SetWorldLocation (Variables|Default|GetDefaultSceneRoot) _newparam false false))))

(event EventSelect
  (bind _m_type (Variables|Default|Getm_Type))
  ;[1 1 1] Cursor and decal handling on selection
  (if (Utilities|Enum|Equal(Enum) (Variables|Default|Getm_State) "E_AVAILABLE")
    (Variables|Default|Setm_State "E_SELECTED")
    (Development|PrintString (Utilities|String|ToString(Name) (Utilities|Name|EnumtoName _m_type)))
    (if (Utilities|Enum|Equal(Enum) _m_type "E_TARGET_GROUND")
      (Variables|/Script/Engine.PlayerController|SetCurrentMouseCursor (Game|GetPlayerController 0) "None")
      (Class|WidgetBlueprintLibrary|SetFocustoGameViewport)
      (CallFunction|SetDecalEnabled true)
      (else
        (Variables|/Script/Engine.PlayerController|SetCurrentMouseCursor (Game|GetPlayerController 0) "CardinalCross")
        (Class|WidgetBlueprintLibrary|SetFocustoGameViewport)))))

(event EventActivate
  ;[1 1 1] Ability activate
  (if (Utilities|Enum|Equal(Enum) (Variables|Default|Getm_Type) "E_TARGET_GROUND")
    (CallFunction|SetDecalEnabled false)))

(fn ConstructionScript)

(fn SetDecalEnabled
  (params (enabled :type Boolean))
  (Rendering|SetVisibility (Variables|Default|GetTargetAreaDecal) enabled false))

(fn ApplyEffecttoUnitsinArea
  (params (Radius :type Float%20%28single-precision%29) (AffectedStat :type EUnitEffectStat%20Enum :default "HEALING") (EffectType :type EUnitEffectType%20Enum :default "OVER_TIME") (Delay :type Float%20%28single-precision%29) (Magnitude :type Integer) (duration :type Integer) (TickParticle :type Particle%20System%20Object%20Reference))
  (bind (_outactors _returnvalue) (Collision|SphereOverlapActors (Transformation|GetWorldLocation (Variables|Default|GetDefaultSceneRoot)) Radius (Utilities|Array|MakeArray "ObjectTypeQuery3") "/Game/RTS/AI/Unit_Character.Unit_Character_C"))
  (if _returnvalue
    (for _array_element _outactors
      (bind _asrts_unit_character (Utilities|Casting|CastToRTS_UnitCharacter _array_element))
      (bind _returnvalue_2 (Class|Ability|CreateUnitEffect AffectedStat EffectType Delay Magnitude duration))
      (Class|UnitEffect|SetTickParticle _returnvalue_2 TickParticle)
      (Class|RTSUnitCharacter|AddUnitEffect _asrts_unit_character _returnvalue_2))))

(fn InitializeDecal
  (params (Radius :type Float%20%28single-precision%29))
  (bind _returnvalue (Class|GameplayStatics|SpawnDecalAttached "/Game/RTS/Blueprints/AblityTests/M_CircleDecal.M_CircleDecal" (Math|Conversions|ToVector(Float) Radius) (Variables|Default|GetDefaultSceneRoot) "None" "0, 0,100.000000" "90.000000, 0, 0" "KeepRelativeOffset" 0.0))
  (Variables|Default|SetTargetAreaDecal _returnvalue)
  (CallFunction|SetDecalEnabled false)
  (Rendering|SetVisibility (Variables|Default|GetDefaultSceneRoot) false true))

(fn ApplyEffecttoTarget
  (params (Target :type RTS%20Unit%20Character%20Object%20Reference) (Affected%20stat :type EUnitEffectStat%20Enum :default "HEALING") (Type :type EUnitEffectType%20Enum :default "OVER_TIME") (Delay :type Float%20%28single-precision%29) (Magnitude :type Integer) (Duration :type Integer) (Tick%20Particle :type Particle%20System%20Object%20Reference))
  (bind _returnvalue (Class|Ability|CreateUnitEffect Affected%20stat Type Delay Magnitude Duration))
  (Class|UnitEffect|SetTickParticle _returnvalue Tick%20Particle)
  (Class|RTSUnitCharacter|AddUnitEffect Target _returnvalue))

(fn ApplyEffecttoArea
  (params (Radius :type Float%20%28single-precision%29) (Affected%20Stat :type EUnitEffectStat%20Enum :default "HEALING") (Type :type EUnitEffectType%20Enum :default "OVER_TIME") (Delay :type Float%20%28single-precision%29) (Magnitude :type Integer) (Duration :type Integer) (Tick%20Particle :type Particle%20System%20Object%20Reference))
  (bind _returnvalue (Game|SpawnActorfromClass "/Game/RTS/Blueprints/AblityTests/AreaOfEffect.AreaOfEffect_C" (Math|Conversions|ToTransform(Vector) (Transformation|GetWorldLocation (Variables|Default|GetDefaultSceneRoot))) "Undefined" 0 Radius Affected%20Stat Type Delay Magnitude Duration 0))
  (Default|SetEffectParticles _returnvalue 0 Tick%20Particle))