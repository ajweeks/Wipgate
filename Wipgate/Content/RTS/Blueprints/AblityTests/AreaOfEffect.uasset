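; Area-of-effect actor for the RTS that applies a timed stat effect to unit characters inside a sphere, with collider and plane sized from Radius.
; Each overlap creates a unit effect with the remaining delay and maps it to its unit; leaving removes it after a brief pause so it can tick.
; Once delay plus duration elapses, Tick removes effects that have ticked and destroys the actor.
; Only the tick particle is forwarded to effects; area particles are unimplemented.
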(event Collision|EventActorBeginOverlap
  (params (OtherActor :type Actor%20Object%20Reference))
  (bind _delay (Variables|Default|GetDelay))
  ;[1 1 1] Create effect for each unit and apply
  (bind _asrts_unit_character (Utilities|Casting|CastToRTS_UnitCharacter OtherActor))
  (bind _returnvalue (Class|GeneralFunctionLibraryCPP|CreateUnitEffect self (Variables|Default|GetEffectStat) (Variables|Default|GetEffectType) (Math|Float|Clamp(Float) (- _delay (Variables|Default|GetElapsed)) 0.0 _delay) (Variables|Default|GetMagnitude) (Variables|Default|GetDuration)))
  (Class|UnitEffect|SetTickParticle _returnvalue (Variables|Default|GetEffectParticle_Tick))
  (Utilities|Map|Add (Variables|Default|GetUnitsAndEffects) _asrts_unit_character _returnvalue)
  (Class|RTSUnitCharacter|AddUnitEffect _asrts_unit_character _returnvalue))

(event Collision|EventActorEndOverlap
  (params (OtherActor :type Actor%20Object%20Reference))
  ;[1 1 1] Remove Effect on end overlap
  (Utilities|FlowControl|Delay 0.01) ; Delay to make sure effect ticks before removing it
  (bind _asrts_unit_character (Utilities|Casting|CastToRTS_UnitCharacter OtherActor))
  (Class|RTSUnitCharacter|RemoveUnitEffect _asrts_unit_character (.Value (Utilities|Map|Find (Variables|Default|GetUnitsAndEffects) _asrts_unit_character))))

(event EventTick
  (params (DeltaSeconds :type Float%20%28single-precision%29))
  ;[1 1 1] Destroy and remove effect after duration
  (bind _output_get (Variables|Default|SetElapsed (+ (Variables|Default|GetElapsed) DeltaSeconds)))
  (if (>= _output_get (Math|Conversions|ToFloat(Integer) (+ (Variables|Default|GetDuration) (Math|Float|Truncate (Variables|Default|GetDelay)))))
    (bind _keys (Utilities|Map|Keys (Variables|Default|GetUnitsAndEffects)))
    (for _array_element _keys
      (if (>= (Variables|/Script/Wipgate.UnitEffect|Getm_Ticks (.Value (Utilities|Map|Find (Variables|Default|GetUnitsAndEffects) _array_element))) 1)
        (Class|RTSUnitCharacter|RemoveUnitEffect _array_element (.Value (Utilities|Map|Find (Variables|Default|GetUnitsAndEffects) _array_element)))))
    (Actor|DestroyActor)))

(fn ConstructionScript
  (bind _radius (Variables|Default|GetRadius))
  (Components|Sphere|SetSphereRadius (Variables|Default|GetSphereCollider) _radius true)
  (Transformation|SetRelativeScale3D (Variables|Default|GetPlane) (* (Math|Conversions|ToVector(Float) _radius) 0.02)))

(fn SetEffectParticles
  (params (Effect%20Start :type Particle%20System%20Object%20Reference) (Effect%20Tick :type Particle%20System%20Object%20Reference) (Effect%20End :type Particle%20System%20Object%20Reference))
  (bind _output_get (Variables|Default|SetEffectParticle_Tick Effect%20Tick))
  (bind _keys (Utilities|Map|Keys (Variables|Default|GetUnitsAndEffects)))
  (for _array_element _keys
    (bind _values (Utilities|Map|Values (Variables|Default|GetUnitsAndEffects)))
    (for _array_element_2 _values
      (Class|UnitEffect|SetTickParticle _array_element_2 _output_get))))

(fn SetAreaParticles)