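; RTS test ability that applies a timed armor effect to units in a targeted ground area.
; On BeginPlay it sets its type to ground-targeted and initializes a targeting decal matching the effect radius.
; On Activate it calls the inherited area-effect function on the ARMOR stat, reusing a speed boost particle as the tick effect, then deselects itself.
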(event Collision|EventActorBeginOverlap
  (params (OtherActor :type Actor%20Object%20Reference)))

(event EventTick
  (params (DeltaSeconds :type Float%20%28single-precision%29))
  (|CallParentFunction DeltaSeconds) ; This node is disabled and will not be called.\nDrag off pins to build functionality.
)

(event EventActivate
  (|CallParentFunction)
  (CallFunction|ApplyEffecttoArea 3e+02 "ARMOR" "OVER_TIME" 0.0 1 5 "/Game/Art/ParticleEffects/SpeedBoost/PE_SpeedBoost.PE_SpeedBoost")
  (Class|Ability|Deselect))

(event EventBeginPlay
  (|CallParentFunction)
  (Variables|Default|Setm_Type "E_TARGET_GROUND")
  (CallFunction|InitializeDecal 3e+02))

(fn ConstructionScript
  (|CallParentFunction))