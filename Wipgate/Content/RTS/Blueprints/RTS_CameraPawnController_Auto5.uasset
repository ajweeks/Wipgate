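; RTS player controller that drives the camera pawn and handles click-and-drag unit selection.
; BeginPlay creates the HUD and draw-box actor; dragging updates a screen-space rectangle or world-space box, depending on UnitSelectionMode.
; Release selects GameState units whose projected bounds corners fall inside the screen rectangle, with Left Shift adding.
; Keys and horizontal screen edges pan at zoom-scaled speed, zoom changes spring arm length, and rotation logic is disconnected.
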(event EventBeginPlay
  ;[1 1 1] Event Begin Play
  (bind _asrts_camera_pawn (Utilities|Casting|CastToRTS_CameraPawn (Game|Player|GetPlayerPawn 0))
    (:then
      (Variables|References|SetCameraPawnRef _asrts_camera_pawn)
      (Variables|References|SetPlayerControllerRef self)
      (Input|SetInputModeGameandUI self 0 "LockAlways" false)
      (bind _returnvalue (UserInterface|CreateWidget "/Game/RTS/Blueprints/Main_UI_HUD.Main_UI_HUD_C" 0 self))
      (Variables|References|SetMainHUD_Ref _returnvalue)
      (Variables|/Game/RTS/Blueprints/Main_UI_HUD.Main_UI_HUD_C|SetCameraPawnController (Variables|References|GetMainHUD_Ref) self)
      (UserInterface|Viewport|AddtoViewport (Variables|References|GetMainHUD_Ref) 0)
      ;[1 1 1] Spawn draw box
      (bind _returnvalue_2 (Game|SpawnActorfromClass "/Script/Engine.Actor" (Math|Transform|MakeTransform "0, 0, 0") "Undefined" 0 0))
      (bind _output_get (Variables|References|SetDrawBoxMesh_Ref _returnvalue_2))
      (AddComponent|AddStaticMeshComponent _output_get false)
      (Rendering|SetActorHiddenInGame _output_get true)
      (Collision|SetActorEnableCollision _output_get false)
      ;[1 1 1] Set game state
      (bind _asrts_game_state (Utilities|Casting|CastToRTS_GameState (Game|GetGameState))
        (:then
          (Variables|References|SetGame%20State _asrts_game_state))
        (:CastFailed
          (Development|PrintString "Failed to cast game state!" true true "(R=1.000000,G=0.015981,B=0.000000,A=1.000000)" 6e+01))))
    (:CastFailed
      (Development|PrintString "Failed to cast camera pawn!" true true "(R=1.000000,G=0.015981,B=0.000000,A=1.000000)" 6e+01))))

(event EventTick
  (params (DeltaSeconds :type Float%20%28single-precision%29))
  (bind _click_start_location_ss (Variables|Default|GetClick%20Start%20Location%20SS))
  (bind _click_end_location_ws (Variables|Default|GetClick%20End%20Location%20WS))
  (bind _click_start_location_ws (Variables|Default|GetClick%20Start%20Location%20WS))
  (bind _mainhud_ref (Variables|References|GetMainHUD_Ref))
  (bind _drawboxmesh_ref (Variables|References|GetDrawBoxMesh_Ref))
  (bind _returnvalue (- _click_end_location_ws _click_start_location_ws))
  (bind _unitselection_ss (Variables|/Game/RTS/Blueprints/Main_UI_HUD.Main_UI_HUD_C|GetUnitSelection_SS _mainhud_ref))
  (bind _rootcomponent (Variables|/Script/Engine.Actor|GetRootComponent _drawboxmesh_ref))
  (bind (_x _y _z) (Math|Vector|BreakVector _returnvalue))
  (bind _returnvalue_2 (Class|WidgetLayoutLibrary|SlotasCanvasSlot _unitselection_ss))
  ;[1 1 1] Click and Drag Box
  (Utilities|FlowControl|Gate true
    (:Exit
      (|SetClickEndLocationSS)
      (|SetClickEndLocationWS)
      (switch int (Variables|Default|GetUnit%20Selection%20Mode) ; Switch based on currently selected camera style
        (:Default
          ;;[1 1 1] 0 - Screen Space
          (Rendering|SetActorHiddenInGame (Variables|References|GetDrawBoxMesh_Ref) true :!label _label)
          (Class|CanvasPanelSlot|SetPosition _returnvalue_2 _click_start_location_ss)
          (Class|CanvasPanelSlot|SetSize _returnvalue_2 (- (Variables|Default|GetClick%20End%20Location%20SS) _click_start_location_ss)))
        (:0
          (goto _label))
        (:1
          ;;[1 1 1] 1 - World Space
          (Transformation|SetWorldLocation _rootcomponent (/ (+ _click_end_location_ws _click_start_location_ws) 2.0) false false)
          (Transformation|SetWorldScale3D _rootcomponent (Math|Vector|MakeVector (* _x 0.01) (* _y 0.01) _z)))))))

(event Input|ActionEvents|InputActionZoomIn
  (params (Key :type Key%20Structure))
  (bind _camerapawnref (Variables|References|GetCameraPawnRef))
  (bind _springarm (Variables|/Game/RTS/Blueprints/RTS_CameraPawn.RTS_CameraPawn_C|GetSpringArm _camerapawnref))
  ;[1 1 1] Camera Controller
  ;;[1 1 1] Zoom
  (:Pressed
    (Variables|/Script/Engine.SpringArmComponent|SetTargetArmLength _springarm (Math|Float|Clamp(Float) (- (Variables|/Script/Engine.SpringArmComponent|GetTargetArmLength _springarm) (Variables|Default|GetZoom%20Sensitivity)) 5e+02 (Variables|Default|GetMax%20Arm%20Distance)))))

(event Input|ActionEvents|InputActionMoveFast
  (params (Key :type Key%20Structure))
  ;[1 1 1] Camera Controller
  ;;[1 1 1] Move Fast
  (:Pressed
    (Variables|Default|SetFastMoveMultiplier (Variables|Default|GetFastMoveSpeed)))
  (:Released
    (Variables|Default|SetFastMoveMultiplier 1.0)))

(event Input|ActionEvents|InputActionZoomOut
  (params (Key :type Key%20Structure))
  (bind _camerapawnref (Variables|References|GetCameraPawnRef))
  (bind _springarm (Variables|/Game/RTS/Blueprints/RTS_CameraPawn.RTS_CameraPawn_C|GetSpringArm _camerapawnref))
  ;[1 1 1] Camera Controller
  ;;[1 1 1] Zoom
  (:Pressed
    (Variables|/Script/Engine.SpringArmComponent|SetTargetArmLength _springarm (Math|Float|Clamp(Float) (+ (Variables|/Script/Engine.SpringArmComponent|GetTargetArmLength _springarm) (Variables|Default|GetZoom%20Sensitivity)) 5e+02 (Variables|Default|GetMax%20Arm%20Distance)))))

(event Input|ActionEvents|InputActionMainClick
  (params (Key :type Key%20Structure))
  (bind _returnvalue (Game|GetPlayerController 0))
  (bind _returnvalue_2 (== "LeftMouseButton" Key))
  (bind _array (Utilities|Array|MakeArray "ObjectTypeQuery1"))
  (bind _self self)
  (bind _game_state (Variables|References|GetGame%20State))
  (bind (_hitresult _returnvalue_3) (Class|PlayerController|GetHitResultUnderCursorforObjects _array true))
  (bind (_locationx _locationy) (Class|WidgetLayoutLibrary|GetMousePositionScaledbyDPI _returnvalue))
  (bind _selected_units (Variables|/Game/RTS/Blueprints/RTS_GameState.RTS_GameState_C|GetSelected%20Units _game_state))
  (bind (_bblockinghit _binitialoverlap _time _distance _location _impactpoint _normal _impactnormal _physmat _hitactor) (Collision|BreakHitResult _hitresult))
  ;[1 1 1] Mouse click handler
  (:Pressed
    (if _returnvalue_2
      (Variables|Default|SetClick%20Start%20Location%20SS (Math|Vector2D|MakeVector2D _locationx _locationy))
      (if (!= _hitactor (Variables|References|GetDrawBoxMesh_Ref))
        (if _returnvalue_3
          (Variables|Default|SetClick%20Start%20Location%20WS (+ "0,0.000000,1.000000" _location))))))
  (:Released
    (if _returnvalue_2
      (Rendering|SetActorHiddenInGame (Variables|References|GetDrawBoxMesh_Ref) true)
      (Class|CanvasPanelSlot|SetSize (Class|WidgetLayoutLibrary|SlotasCanvasSlot (Variables|/Game/RTS/Blueprints/Main_UI_HUD.Main_UI_HUD_C|GetUnitSelection_SS (Variables|References|GetMainHUD_Ref))))
      ;[1 1 1] Unit selection
      (if (Game|Player|IsInputKeyDown (Game|GetPlayerController 0) "LeftShift")
        _
        (else
          (for _array_element _selected_units
            (Default|SetSelected _array_element false))
          (Utilities|Array|Clear _selected_units)))
      (for _array_element_2 (Variables|/Game/RTS/Blueprints/RTS_GameState.RTS_GameState_C|GetAll%20Units (Variables|References|GetGame%20State))
        ;;[1 1 1] Box-Point Check
        (if (Variables|/Game/RTS/Blueprints/Unit_Character.Unit_Character_C|GetShow%20Selection%20Box _array_element_2)
          (Rendering|Debug|DrawDebugBox (.Location (Math|Transform|BreakTransform (Transformation|GetActorTransform _array_element_2))) (Variables|/Game/RTS/Blueprints/Unit_Character.Unit_Character_C|GetSelection%20Box%20Size _array_element_2) "(R=5.000000,G=5.000000,B=5.000000,A=1.000000)" "0, 0, 0" 2.5 4.0)
          (bind _point_in_bounds (CallFunction|PointinBounds2D (.ScreenPosition (Class|WidgetLayoutLibrary|ProjectWorldLocationtoWidgetPosition _self (- (.Location (Math|Transform|BreakTransform (Transformation|GetActorTransform _array_element_2))) (Variables|/Game/RTS/Blueprints/Unit_Character.Unit_Character_C|GetSelection%20Box%20Size _array_element_2)))) (Math|Vector4|MakeVector4 (.X (Math|Vector2D|BreakVector2D (.Vector%20Min (Utilities|Vector2DMinMax (Variables|Default|GetClick%20Start%20Location%20SS) (Variables|Default|GetClick%20End%20Location%20SS))))) (.Y (Math|Vector2D|BreakVector2D (.Vector%20Min (Utilities|Vector2DMinMax (Variables|Default|GetClick%20Start%20Location%20SS) (Variables|Default|GetClick%20End%20Location%20SS))))) (.X (Math|Vector2D|BreakVector2D (.Vector%20Max (Utilities|Vector2DMinMax (Variables|Default|GetClick%20Start%20Location%20SS) (Variables|Default|GetClick%20End%20Location%20SS))))) (.Y (Math|Vector2D|BreakVector2D (.Vector%20Max (Utilities|Vector2DMinMax (Variables|Default|GetClick%20Start%20Location%20SS) (Variables|Default|GetClick%20End%20Location%20SS))))))))
          (bind _point_in_bounds_2 (CallFunction|PointinBounds2D (.ScreenPosition (Class|WidgetLayoutLibrary|ProjectWorldLocationtoWidgetPosition _self (+ (.Location (Math|Transform|BreakTransform (Transformation|GetActorTransform _array_element_2))) (Variables|/Game/RTS/Blueprints/Unit_Character.Unit_Character_C|GetSelection%20Box%20Size _array_element_2)))) (Math|Vector4|MakeVector4 (.X (Math|Vector2D|BreakVector2D (.Vector%20Min (Utilities|Vector2DMinMax (Variables|Default|GetClick%20Start%20Location%20SS) (Variables|Default|GetClick%20End%20Location%20SS))))) (.Y (Math|Vector2D|BreakVector2D (.Vector%20Min (Utilities|Vector2DMinMax (Variables|Default|GetClick%20Start%20Location%20SS) (Variables|Default|GetClick%20End%20Location%20SS))))) (.X (Math|Vector2D|BreakVector2D (.Vector%20Max (Utilities|Vector2DMinMax (Variables|Default|GetClick%20Start%20Location%20SS) (Variables|Default|GetClick%20End%20Location%20SS))))) (.Y (Math|Vector2D|BreakVector2D (.Vector%20Max (Utilities|Vector2DMinMax (Variables|Default|GetClick%20Start%20Location%20SS) (Variables|Default|GetClick%20End%20Location%20SS))))))))
          (if (or _point_in_bounds _point_in_bounds_2)
            (Default|SetSelected _array_element_2 true)
            (Utilities|Array|AddUnique (Variables|/Game/RTS/Blueprints/RTS_GameState.RTS_GameState_C|GetSelected%20Units (Variables|References|GetGame%20State)) _array_element_2)
            (elif (not (Game|Player|IsInputKeyDown (Game|GetPlayerController 0) "LeftShift"))
              (Default|SetSelected _array_element_2 false)
              (Utilities|Array|RemoveItem (Variables|/Game/RTS/Blueprints/RTS_GameState.RTS_GameState_C|GetSelected%20Units (Variables|References|GetGame%20State)) _array_element_2))))))))

(event Input|AxisEvents|InputAxisMoveRight
  (params (AxisValue :type Float%20%28single-precision%29))
  (bind _movesensitivity (CallFunction|MovementSpeedCalculation))
  (bind _fastmovemultiplier (Variables|Default|GetFastMoveMultiplier))
  (bind _camerapawnref (Variables|References|GetCameraPawnRef))
  (bind _transform (Utilities|MovementDirection "-0.700000,0.700000,0.000000" AxisValue _movesensitivity _fastmovemultiplier _camerapawnref))
  (bind (_location _rotation _scale) (Math|Transform|BreakTransform _transform))
  (bind (_x _y) (Math|Vector|BreakVector _location))
  ;[1 1 1] Camera Controller
  ;;[1 1 1] Keyboard Movement
  (if (not (Variables|Default|GetDisableCamNav))
    (Transformation|SetActorTransform _camerapawnref (Math|Transform|MakeTransform (Math|Vector|MakeVector _x _y 1e+02) _rotation _scale))))

(event Input|AxisEvents|InputAxisMoveForward
  (params (AxisValue :type Float%20%28single-precision%29))
  (bind _camerapawnref (Variables|References|GetCameraPawnRef))
  ;[1 1 1] Camera Controller
  ;;[1 1 1] Keyboard Movement
  (if (not (Variables|Default|GetDisableCamNav))
    (Transformation|SetActorTransform _camerapawnref (Utilities|MovementDirection "0.700000,0.700000,0.000000" AxisValue (CallFunction|MovementSpeedCalculation) (Variables|Default|GetFastMoveMultiplier) _camerapawnref))))

(event Input|MouseEvents|MouseY
  (params (AxisValue :type Float%20%28single-precision%29))
  ;[1 1 1] Camera Controller
  ;;[1 1 1] Rotation (DISABLED)
  (Utilities|FlowControl|Gate true))

(event Input|MouseEvents|MouseX
  (params (AxisValue :type Float%20%28single-precision%29))
  (bind _returnvalue (Viewport|GetViewportSize))
  (bind (_locationx _locationy) (Game|Player|GetMousePosition))
  (bind _movesensitivity (CallFunction|MovementSpeedCalculation))
  (bind _fastmovemultiplier (Variables|Default|GetFastMoveMultiplier))
  (bind _camerapawnref (Variables|References|GetCameraPawnRef))
  (bind _edgesize (Variables|Default|GetEdgeSize))
  (bind (_x _y) (Math|Vector2D|BreakVector2D _returnvalue))
  (bind _returnvalue_2 (/ _locationx _x))
  ;[1 1 1] Camera Controller
  ;;[1 1 1] Edge Movement
  (if (not (Variables|Default|GetDisableCamNav))
    (if (>= _returnvalue_2 (- 1.0 _edgesize))
      (Transformation|SetActorTransform _camerapawnref (Utilities|MovementDirection "0.700000,0.700000,0.000000" AxisValue _movesensitivity _fastmovemultiplier _camerapawnref)))
    (if (<= _returnvalue_2 _edgesize)
      (Transformation|SetActorTransform _camerapawnref (Utilities|MovementDirection "-0.700000,0.700000,0.000000" (stale Input|MouseEvents|MouseY AxisValue) _movesensitivity _fastmovemultiplier _camerapawnref)))))

(event Input|MouseEvents|MouseY
  (params (AxisValue :type Float%20%28single-precision%29))
  ;[1 1 1] Camera Controller
  ;;[1 1 1] Edge Movement
  (if (Variables|Default|GetDisableCamNav)
    _))

(event Input|MouseEvents|MouseX
  (params (AxisValue :type Float%20%28single-precision%29))
  ;[1 1 1] Camera Controller
  ;;[1 1 1] Rotation (DISABLED)
  (Utilities|FlowControl|Gate true))

(event Input|MouseEvents|LeftMouseButton
  (params (Key :type Key%20Structure))
  (bind _click_start_location_ss (Variables|Default|GetClick%20Start%20Location%20SS))
  (bind _click_end_location_ws (Variables|Default|GetClick%20End%20Location%20WS))
  (bind _click_start_location_ws (Variables|Default|GetClick%20Start%20Location%20WS))
  (bind _mainhud_ref (Variables|References|GetMainHUD_Ref))
  (bind _drawboxmesh_ref (Variables|References|GetDrawBoxMesh_Ref))
  (bind _drawboxmesh_ref_2 (Variables|References|GetDrawBoxMesh_Ref))
  (bind _returnvalue (- _click_end_location_ws _click_start_location_ws))
  (bind _unitselection_ss (Variables|/Game/RTS/Blueprints/Main_UI_HUD.Main_UI_HUD_C|GetUnitSelection_SS _mainhud_ref))
  (bind _rootcomponent (Variables|/Script/Engine.Actor|GetRootComponent _drawboxmesh_ref))
  (bind (_x _y _z) (Math|Vector|BreakVector _returnvalue))
  (bind _returnvalue_2 (Class|WidgetLayoutLibrary|SlotasCanvasSlot _unitselection_ss))
  ;[1 1 1] Click and Drag Box
  (:Pressed
    (Rendering|SetActorHiddenInGame _drawboxmesh_ref_2 false)
    (Utilities|FlowControl|Gate true) ; enters at Open
  )
  (:Released
    (Rendering|SetActorHiddenInGame _drawboxmesh_ref_2 true)
    (Utilities|FlowControl|Gate true) ; enters at Close
  ))

(fn ConstructionScript)

(fn MovementSpeedCalculation
  (return (Math|Float|Clamp(Float) (/ (Variables|/Script/Engine.SpringArmComponent|GetTargetArmLength (Variables|/Game/RTS/Blueprints/RTS_CameraPawn.RTS_CameraPawn_C|GetSpringArm (Variables|References|GetCameraPawnRef))) 3e+02) 1.0 2e+01)))

(fn PointinBounds2D
  (params (Point :type Vector%202D%20Structure) (Bounds :type Vector%204%20Structure))
  (bind (_x _y _z _w) (Math|Vector4|BreakVector4 Bounds))
  (bind (_x_2 _y_2) (Math|Vector2D|BreakVector2D Point))
  (return (and (and (> _x_2 _x) (> _y_2 _y)) (and (< _x_2 _z) (< _y_2 _w)))))

(fn BoxesOverlap
  (params (Box1%20Min :type Vector%202D%20Structure) (Box1%20Max :type Vector%202D%20Structure) (Box2%20Min :type Vector%202D%20Structure) (Box2%20Max :type Vector%202D%20Structure))
  (bind (_x _y) (Math|Vector2D|BreakVector2D Box2%20Max))
  (bind (_x_2 _y_2) (Math|Vector2D|BreakVector2D Box1%20Min))
  (bind (_x_3 _y_3) (Math|Vector2D|BreakVector2D Box1%20Max))
  (bind (_x_4 _y_4) (Math|Vector2D|BreakVector2D Box2%20Min))
  (return (and (or (and (< _x_2 _x) (> _x_2 _x_4)) (and (> _x_3 _x_4) (< _x_3 _x))) (or (and (> _y_2 _y) (< _y_2 _y_4)) (and (< _y_3 _y_4) (> _y_3 _y))))))