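; Ground-targeted healing ability for an RTS, built as a child of a parent ability class.
; On BeginPlay it sets the ground target type and initializes a targeting decal with the same radius as its effect.
; On activation it applies a timed effect to units in that area, with start, tick, constant and end particles, then deselects itself.
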(event EventBeginPlay
  (|CallParentFunction)
  (Variables|Default|SetType "E_TARGET_GROUND")
  (CallFunction|InitializeDecal 5e+02))

(event Collision|EventActorBeginOverlap
  (params (OtherActor :type Actor%20Object%20Reference)))

(event EventTick
  (params (DeltaSeconds :type Float%20%28single-precision%29))
  (|CallParentFunction DeltaSeconds) ; This node is disabled and will not be called.\nDrag off pins to build functionality.
)

(event EventActivate
  (|CallParentFunction)
  (CallFunction|ApplyEffecttoUnitsinArea 5e+02 "HEALING" "OVER_TIME" 0.0 50 5 "/Game/Art/ParticleEffects/Heal/PE_Heal.PE_Heal" "/Game/Art/ParticleEffects/Hit/PE_Hit.PE_Hit" "/Game/Art/ParticleEffects/Hit/PE_Hit.PE_Hit" "/Game/Art/ParticleEffects/SpeedBoost/PE_SpeedBoost.PE_SpeedBoost")
  (Class|Ability|Deselect))

(fn ConstructionScript
  (|CallParentFunction))