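; Commander ability for the RTS that provides a passive buff, toggling between an attack buff and a speed buff.
; It spawns the attack buff ability actor on BeginPlay and forwards Passive calls to whichever sub-ability is current.
; Activate destroys the current buff actor and spawns the other, with the speed buff stored in AbilityHealing despite the name.
; Tick keeps the current sub-ability's caster matched to its own.
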(event EventActivate
  (|CallParentFunction)
  (if (== (Variables|Default|GetAbility_Current) (Variables|Default|GetAbility_DamageBuff))
    (Actor|DestroyActor (Variables|Default|GetAbility_DamageBuff))
    (bind _returnvalue (Game|SpawnActorfromClass "/Game/RTS/Blueprints/Ablities/Swap_Passives/Ab_Commander_SpeedBuff.Ab_Commander_SpeedBuff_C" (Math|Transform|MakeTransform "0, 0, 0") "Undefined" 0 0))
    (bind _output_get (Variables|Default|SetAbility_Healing _returnvalue))
    (Variables|Default|SetAbility_Current _output_get)
    (else
      (Actor|DestroyActor (Variables|Default|GetAbility_Healing))
      (bind _returnvalue_2 (Game|SpawnActorfromClass "/Game/RTS/Blueprints/Ablities/Swap_Passives/Ab_Commander_AttackBuff.Ab_Commander_AttackBuff_C" (Math|Transform|MakeTransform "0, 0, 0") "Undefined" 0 0))
      (bind _output_get_2 (Variables|Default|SetAbility_DamageBuff _returnvalue_2))
      (Variables|Default|SetAbility_Current _output_get_2))))

(event EventPassive
  (|CallParentFunction)
  (Class|Ability|Passive (Variables|Default|GetAbility_Current)))

(event EventBeginPlay
  (|CallParentFunction)
  (bind _returnvalue (Game|SpawnActorfromClass "/Game/RTS/Blueprints/Ablities/Swap_Passives/Ab_Commander_AttackBuff.Ab_Commander_AttackBuff_C" (Math|Transform|MakeTransform "0, 0, 0") "Undefined" 0 0))
  (bind _output_get (Variables|Default|SetAbility_DamageBuff _returnvalue))
  (Variables|/Script/Wipgate.Ability|Setm_Caster _output_get (Variables|Default|Getm_Caster))
  (Variables|Default|SetAbility_Current _output_get))

(event EventTick
  (params (DeltaSeconds :type Float%20%28single-precision%29))
  (|CallParentFunction DeltaSeconds)
  (if (!= (Variables|/Script/Wipgate.Ability|Getm_Caster (Variables|Default|GetAbility_Current)) (Variables|Default|Getm_Caster))
    (Variables|/Script/Wipgate.Ability|Setm_Caster (Variables|Default|GetAbility_Current) (Variables|Default|Getm_Caster))))

(fn ConstructionScript
  (|CallParentFunction))