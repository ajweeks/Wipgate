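; Commander leap ability for the RTS that, on activation, sends the casting unit to the ability actor's location.
; On BeginPlay it initializes a decal with a size value through an inherited function.
; Activate runs the parent logic, casts the caster to RTS_UnitCharacter, then issues an AI MoveToLocation with pathfinding disabled.
; The file itself applies no jump, launch or damage logic.
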(event EventActivate
  (bind _m_caster (Variables|Default|Getm_Caster))
  (|CallParentFunction)
  (Utilities|Casting|CastToRTS_UnitCharacter _m_caster)
  (AI|Navigation|MovetoLocation (AI|GetAIController _m_caster) (Transformation|GetWorldLocation (Variables|Default|GetDefaultSceneRoot)) -1.0 true false false))

(event EventBeginPlay
  (|CallParentFunction)
  (CallFunction|InitializeDecal 3e+02))

(fn ConstructionScript
  (|CallParentFunction))