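; RTS player controller that turns right-clicks into orders for selected units and handles specialist ability buttons.
; A cursor trace makes a living unit the forced target; other hits become forced moves if navigable, with a click effect, otherwise an invalid sound.
; Orders go through each unit's AI_UnitController, using selection from the game state.
; Ability buttons read the first selected specialist, activating self-type abilities immediately and storing and selecting others.
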(event EventOnAbilityPassiveButtonPress
  (bind _asrts_game_state_bp (Utilities|Casting|CastToRTS_GameState_BP (Game|GetGameState)))
  (bind _asspecialist_character (Utilities|Casting|CastToSpecialist_Character (Utilities|Array|Get(acopy) (Variables|/Script/Wipgate.RTS_GameState|GetSelectedUnits _asrts_game_state_bp))))
  (if (Utilities|Enum|Equal(Enum) (Variables|/Script/Wipgate.Ability|GetType (Variables|/Game/RTS/AI/Specialist_Character.Specialist_Character_C|GetAbility_Passive _asspecialist_character)) "E_SELF")
    (Class|Ability|Activate (Variables|/Game/RTS/AI/Specialist_Character.Specialist_Character_C|GetAbility_Passive _asspecialist_character))
    (else
      (bind _output_get (Variables|Default|Setm_SelectedAbility (Variables|/Game/RTS/AI/Specialist_Character.Specialist_Character_C|GetAbility_Passive _asspecialist_character)))
      (Class|Ability|Select _output_get))))

(event EventOnAbilityConstructButtonPress
  (bind _asrts_game_state_bp (Utilities|Casting|CastToRTS_GameState_BP (Game|GetGameState)))
  (bind _asspecialist_character (Utilities|Casting|CastToSpecialist_Character (Utilities|Array|Get(acopy) (Variables|/Script/Wipgate.RTS_GameState|GetSelectedUnits _asrts_game_state_bp))))
  (if (Utilities|Enum|Equal(Enum) (Variables|/Script/Wipgate.Ability|GetType (Variables|/Game/RTS/AI/Specialist_Character.Specialist_Character_C|GetAbility_Construct _asspecialist_character)) "E_SELF")
    (Class|Ability|Activate (Variables|/Game/RTS/AI/Specialist_Character.Specialist_Character_C|GetAbility_Construct _asspecialist_character))
    (else
      (bind _output_get (Variables|Default|Setm_SelectedAbility (Variables|/Game/RTS/AI/Specialist_Character.Specialist_Character_C|GetAbility_Construct _asspecialist_character)))
      (Class|Ability|Select _output_get))))

(event EventOnAbilityActiveButtonPress
  (bind _asrts_game_state_bp (Utilities|Casting|CastToRTS_GameState_BP (Game|GetGameState)))
  (bind _asspecialist_character (Utilities|Casting|CastToSpecialist_Character (Utilities|Array|Get(acopy) (Variables|/Script/Wipgate.RTS_GameState|GetSelectedUnits _asrts_game_state_bp))))
  (if (Utilities|Enum|Equal(Enum) (Variables|/Script/Wipgate.Ability|GetType (Variables|/Game/RTS/AI/Specialist_Character.Specialist_Character_C|GetAbility_Active _asspecialist_character)) "E_SELF")
    (Class|Ability|Activate (Variables|/Game/RTS/AI/Specialist_Character.Specialist_Character_C|GetAbility_Active _asspecialist_character))
    (else
      (bind _output_get (Variables|Default|Setm_SelectedAbility (Variables|/Game/RTS/AI/Specialist_Character.Specialist_Character_C|GetAbility_Active _asspecialist_character)))
      (Class|Ability|Select _output_get))))

(event Input|ActionEvents|InputActionSecondaryClick
  (params (Key :type Key%20Structure))
  (bind _returnvalue (Game|GetPlayerController 0))
  (bind _hitresult (Game|Player|GetHitResultUnderCursorbyChannel _returnvalue "TraceTypeQuery2" true))
  (bind (_bblockinghit _binitialoverlap _time _distance _location _impactpoint _normal _impactnormal _physmat _hitactor) (Collision|BreakHitResult _hitresult))
  ;[1 1 1] Right-click movement
  ;;[1 1 1] Get Gamestate on right mouse
  (:Pressed
    (bind _asrts_game_state_bp (Utilities|Casting|CastToRTS_GameState_BP (Game|GetGameState)))
    ;;[1 1 1] Check if user has units selected
    (if (> (Utilities|Array|Length (Variables|/Script/Wipgate.RTS_GameState|GetSelectedUnits _asrts_game_state_bp)) 0)
      ;;[1 1 1] Raycast from mouse
      (bind _asunit_character (Utilities|Casting|CastToUnit_Character _hitactor)
        (:then
          ;;[1 1 1] If selection was character
          (if (not (Variables|/Script/Wipgate.RTS_UnitCoreComponent|GetIsDead (Variables|/Game/RTS/AI/Unit_Character.Unit_Character_C|GetUnit_Core_Component _asunit_character)))
            (for _array_element (Variables|/Script/Wipgate.RTS_GameState|GetSelectedUnits _asrts_game_state_bp)
              (if (!= _array_element _asunit_character)
                (bind _asai_unit_controller (Utilities|Casting|CastToAI_UnitController (AI|GetAIController _array_element)))
                (Default|SetTargetActor _asai_unit_controller _asunit_character false true)))
            (else
              (if (.ReturnValue (AI|Navigation|ProjectPointtoNavigation _location 0 0 "0, 0, 0")) :!label _label
                ;;[1 1 1] If selection was non-character
                (for _array_element_2 (Variables|/Script/Wipgate.RTS_GameState|GetSelectedUnits _asrts_game_state_bp)
                  (bind _asai_unit_controller_2 (Utilities|Casting|CastToAI_UnitController (AI|GetAIController _array_element_2)))
                  (Default|SetTargetLocation _asai_unit_controller_2 _location true))
                (Game|SpawnActorfromClass "/Game/Art/ParticleEffects/ClickEffect/BP_ClickEffect.BP_ClickEffect_C" (Math|Conversions|ToTransform(Vector) _location) "AlwaysSpawn" 0 (Variables|Default|GetLocation_Click_Color) (Variables|Default|GetLocation_Click_Speed) 0)
                (else
                  (Audio|PlaySound2D (Variables|Default|GetLocation_Click_InvalidSound)))))))
        (:CastFailed
          (goto _label))))))

(fn ConstructionScript)