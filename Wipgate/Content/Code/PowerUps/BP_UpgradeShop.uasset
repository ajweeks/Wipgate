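; BP_UpgradeShop is a shop zone offering three purchasable upgrades when player units are inside and aggressive AI units are absent.
; On BeginPlay it spawns BP_PurchasablePowerUp actors from random data table rows at rotated offsets, then collects those overlapping its cube.
; Each Tick it checks RTS_Entity team alignments in the cube to show or hide items and recolor the zone's dynamic material.
; An entry sound plays when the shop becomes active.
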(event EventBeginPlay
  (CallFunction|SpawnItems)
  (bind _returnvalue (Rendering|Material|CreateDynamicMaterialInstance (Variables|Default|GetOverlapCube) 0 "/Game/Art/PowerUps/PickUps/M_ShopZone.M_ShopZone" :!class /Script/Engine.PrimitiveComponent))
  (Variables|Default|SetZoneMatInstance _returnvalue))

(event EventTick
  (params (DeltaSeconds :type Float%20%28single-precision%29))
  (CallFunction|CheckBoxOverlap)
  (CallFunction|UpdateColors)
  (for _array_element (Variables|Default|GetShopItems)
    (if (Utilities|IsValid _array_element)
      (Default|SetHidden _array_element (not (and (Variables|Default|GetFriendliesInRange) (not (Variables|Default|GetEnemiesInRange))))))))

(fn ConstructionScript
  (Transformation|AttachComponentToComponent (Variables|Default|GetHat) (Variables|Default|GetSkeletalMesh) "HeadTop_End" "KeepRelative" "KeepRelative" "KeepRelative" true))

(fn SpawnItems
  (CallFunction|SpawnPurchaseableUpgrade "-370.000000,-200.000000, 0")
  (CallFunction|SpawnPurchaseableUpgrade "-320.000000,-30.000000, 0")
  (CallFunction|SpawnPurchaseableUpgrade "-360.000000,110.000000, 0")
  (for _array_element (Collision|GetOverlappingActors (Variables|Default|GetOverlapCube) "/Game/Code/PowerUps/BP_PurchasablePowerUp.BP_PurchasablePowerUp_C" :!class /Script/Engine.PrimitiveComponent)
    (bind _asbp_purchasable_power_up (Utilities|Casting|CastToBP_PurchasablePowerUp _array_element))
    (Utilities|Array|Add (Variables|Default|GetShopItems) _asbp_purchasable_power_up)))

(fn GetRandomUpgrade
  (bind _outrownames (DataTable|GetDataTableRowNames (Variables|Default|GetUpradeDataTable)))
  (bind _returnvalue (Utilities|GetDataTableRow (Variables|Default|GetUpradeDataTable) (Utilities|Array|Get(acopy) _outrownames (Math|Random|RandomInteger (Utilities|Array|Length _outrownames))))
    (:then
      (return _returnvalue))))

(fn SpawnPurchaseableUpgrade
  (params (InputOffset :type Vector))
  (bind _newparam (CallFunction|GetRandomUpgrade))
  (bind _returnvalue (Game|SpawnActorfromClass "/Game/Code/PowerUps/BP_PurchasablePowerUp.BP_PurchasablePowerUp_C" (Math|Transform|MakeTransform (+ (Transformation|GetActorLocation) (Math|Vector|RotateVector InputOffset (Transformation|GetActorRotation)))) "Undefined" 0 (.Price (Utilities|Struct|BreakUpgradeRow _newparam)) (.Description (Utilities|Struct|BreakUpgradeRow _newparam)) (.Title (Utilities|Struct|BreakUpgradeRow _newparam)) (.Color (Utilities|Struct|BreakUpgradeRow _newparam)) (.Upgrades (Utilities|Struct|BreakUpgradeRow _newparam)) (.Texture (Utilities|Struct|BreakUpgradeRow _newparam)) 0))
  (Variables|/Game/Code/PowerUps/BP_PurchasablePowerUp.BP_PurchasablePowerUp_C|SetUpgrade%20Shop _returnvalue self))

(fn CheckBoxOverlap
  (Variables|Default|SetEnemiesInRange false)
  (Variables|Default|SetFriendliesInRange false)
  (for _array_element (Collision|GetOverlappingActors (Variables|Default|GetOverlapCube) "/Script/Wipgate.RTS_Entity" :!class /Script/Engine.PrimitiveComponent)
    (bind _asrts_entity (Utilities|Casting|CastToRTS_Entity _array_element))
    (if (Utilities|Enum|Equal(Enum) (Variables|/Script/Wipgate.RTS_Team|GetAlignment (Variables|/Script/Wipgate.RTS_Entity|GetTeam _asrts_entity)) "E_PLAYER")
      (Variables|Default|SetFriendliesInRange true)
      (elif (Utilities|Enum|Equal(Enum) (Variables|/Script/Wipgate.RTS_Team|GetAlignment (Variables|/Script/Wipgate.RTS_Entity|GetTeam _asrts_entity)) "E_AGGRESSIVE_AI")
        (Variables|Default|SetEnemiesInRange true)))))

(fn UpdateColors
  (if (Variables|Default|GetEnemiesInRange)
    (Rendering|Material|SetVectorParameterValue (Variables|Default|GetZoneMatInstance) "Color" "(R=1.000000,G=0.006586,B=0.000000,A=1.000000)" :!class /Script/Engine.MaterialInstanceDynamic)
    (Variables|Default|SetWasShopActive false)
    (elif (Variables|Default|GetFriendliesInRange)
      (Rendering|Material|SetVectorParameterValue (Variables|Default|GetZoneMatInstance) "Color" "(R=0.082624,G=1.000000,B=0.000000,A=1.000000)" :!class /Script/Engine.MaterialInstanceDynamic)
      (if (not (Variables|Default|GetWasShopActive))
        (Variables|Default|SetWasShopActive true)
        (Audio|PlaySoundatLocation "/Game/Art/Sounds/Shop/ShopEntry_Cue.ShopEntry_Cue" (Transformation|GetActorLocation) "0, 0, 0" 1.0 1.0 0.0 "/Game/Art/Sounds/SA_EffectSounds.SA_EffectSounds" "/Game/Art/Sounds/SCo_EffectSounds.SCo_EffectSounds"))
      (else
        (Rendering|Material|SetVectorParameterValue (Variables|Default|GetZoneMatInstance) "Color" "(R=1.000000,G=1.000000,B=1.000000,A=1.000000)" :!class /Script/Engine.MaterialInstanceDynamic)
        (Variables|Default|SetWasShopActive false)))))