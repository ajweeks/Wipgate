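; Shop power-up actor that the player clicks to buy upgrades for their team with Luma.
; Hovering shows a highlight plane and shop cursor, then an info popup after a delay.
; An affordable click spends Luma and starts a Tick-driven disappearance that animates the sphere material.
; When it finishes, it spawns cost-scaled particles, adds the upgrades, plays a sound, destroys itself and leaves the shop's item list.
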(event OnBeginCursorOver(Sphere)
  (params (TouchedComponent :type Primitive%20Component%20Object%20Reference))
  (bind _returnvalue (Game|GetPlayerController 0))
  (bind _asrts_player_controller_bp (Utilities|Casting|CastToRTS_PlayerController_BP _returnvalue))
  (bind _cursorref (Variables|/Script/Wipgate.RTS_PlayerController|GetCursorRef _asrts_player_controller_bp))
  ;[1 1 1] Cursor Over Begin/End
  (if (not (or (Variables|Default|GetHidden) (Variables|Default|GetDisappearing)))
    (Variables|Default|SetHovering true)
    (Rendering|SetVisibility (Variables|Default|GetPlane) true false)
    (if (not (Utilities|IsValid (Variables|/Script/Wipgate.RTS_PlayerController|GetSelectedAbility _asrts_player_controller_bp)))
      (Class|RTSCursor|SetCursorTexture _cursorref (Variables|/Script/Wipgate.RTS_Cursor|GetShopTexture _cursorref)))))

(event OnEndCursorOver(Sphere)
  (params (TouchedComponent :type Primitive%20Component%20Object%20Reference))
  (bind _returnvalue (Game|GetPlayerController 0))
  (bind _asrts_player_controller_bp (Utilities|Casting|CastToRTS_PlayerController_BP _returnvalue))
  (bind _cursorref (Variables|/Script/Wipgate.RTS_PlayerController|GetCursorRef _asrts_player_controller_bp))
  ;[1 1 1] Cursor Over Begin/End
  (if (not (Variables|Default|GetHidden))
    (Variables|Default|SetHovering false)
    (Rendering|SetVisibility (Variables|Default|GetScreen%20UI) false true)
    (Variables|Default|SetHover%20Time 0.0)
    (Rendering|SetVisibility (Variables|Default|GetPlane) false false)
    (if (== (Variables|/Script/Wipgate.RTS_Cursor|GetShopTexture _cursorref) (Variables|/Script/Wipgate.RTS_Cursor|GetCurrentTexture _cursorref))
      (Class|RTSCursor|SetCursorTexture _cursorref (Variables|/Script/Wipgate.RTS_Cursor|GetDefaultTexture _cursorref)))))

(event OnClicked(Sphere)
  (params (TouchedComponent :type Primitive%20Component%20Object%20Reference) (ButtonPressed :type Key%20Structure))
  ;[1 1 1] On Sphere Clicked
  (if (not (Variables|Default|GetHidden))
    (bind _asrts_player_controller_bp (Utilities|Casting|CastToRTS_PlayerController_BP (Game|GetPlayerController 0)))
    (bind _returnvalue (Class|RTSPlayerController|GetCurrentLumaAmount _asrts_player_controller_bp))
    (if (>= _returnvalue (Variables|Default|GetCost))
      (Class|RTSPlayerController|SpendLuma _asrts_player_controller_bp (Variables|Default|GetCost))
      (Variables|Default|SetIs%20Disappearing true)
      (else
        ;;[1 1 1] If player cant afford upgrade
        (Development|PrintString "YOU CANT AFFORD THIS ITEM" true true "(R=1.000000,G=0.006282,B=0.000000,A=1.000000)")
        (Audio|SpawnSound2D "/Game/Art/Sounds/Shop/SW_CantAffordItem_Cue.SW_CantAffordItem_Cue" 1.0 1.5 0.0 "/Game/Art/Sounds/SCo_EffectSounds.SCo_EffectSounds")))))

(event EventBeginPlay
  ;[1 1 1] On Begin Play
  (|CallParentFunction)
  (bind _asui_power_up_pop_up_info (Utilities|Casting|CastToUI_PowerUpPopUpInfo (UserInterface|GetUserWidgetObject (Variables|Default|GetScreen%20UI))))
  (Default|SetVariables _asui_power_up_pop_up_info (Utilities|Text|ToText(String) (Utilities|String|ToString(Name) (Variables|Default|GetName))) (Utilities|Text|ToText(String) (Variables|Default|GetDescription)) (Variables|Default|GetCardIcon) (Variables|Default|GetColor)))

(event EventTick
  (params (DeltaSeconds :type Float%20%28single-precision%29))
  ;[1 1 1] Tick
  (|CallParentFunction DeltaSeconds)
  (Utilities|FlowControl|Sequence
    (:then_0
      (if (Variables|Default|GetHovering)
        (bind _output_get (Variables|Default|SetHover%20Time (+ (Variables|Default|GetHover%20Time) (Utilities|Time|GetWorldDeltaSeconds))))
        (Math|Float|CompareFloat _output_get (Variables|Default|GetScreen%20UI%20Display%20Delay)
          (:>
            (Rendering|SetVisibility (Variables|Default|GetScreen%20UI) true true)))))
    (:then_1
      (if (Variables|Default|GetIs%20Disappearing)
        (CallFunction|Disappear)))))

(event EventDisappear
  ;[1 1 1] Disappear
  (Variables|Default|SetDisappearing true)
  (Variables|Default|SetDisappearanceTimer (+ (Variables|Default|GetDisappearanceTimer) (Utilities|Time|GetWorldDeltaSeconds)))
  (Math|Float|CompareFloat (Variables|Default|GetDisappearanceTimer) (/ (Variables|Default|GetDisappearanceDuration) 2.0)
    (:>
      (Rendering|SetVisibility (Variables|Default|GetMaterialBillboard) false false))
    (:==
      (Rendering|Material|SetScalarParameterValue (Variables|Default|GetSphereMatIntance) "TransitionTime" (/ (Variables|Default|GetDisappearanceTimer) (/ (Variables|Default|GetDisappearanceDuration) 2.0)) :!class /Script/Engine.MaterialInstanceDynamic :!label _label))
    (:<
      (goto _label)))
  ;;[1 1 1] Destroy
  (Math|Float|CompareFloat (Variables|Default|GetDisappearanceTimer) (Variables|Default|GetDisappearanceDuration)
    (:>
      (Rendering|SetVisibility (Variables|Default|GetPointLight) false true)
      (bind _returnvalue (Effects|SpawnEmitteratLocation "/Game/Art/ParticleEffects/Pickup/PE_PickUp.PE_PickUp" (Transformation|GetWorldLocation (Variables|Default|GetSphere))))
      (Effects|Components|ParticleSystem|SetFloatParameter _returnvalue "SpawnRate" (Math|Conversions|ToFloat(Integer) (/ (Variables|Default|GetCost) 10)))
      (Development|PrintString (Utilities|String|Append "Add \"" (Utilities|String|ToString(Name) (Variables|Default|GetName)) "\" to obtained powerups.") true true "(R=1.000000,G=0.000000,B=0.783689,A=1.000000)")
      (bind _asrts_player_controller (Utilities|Casting|CastToRTS_PlayerController (Game|GetPlayerController 0)))
      (Class|RTSTeam|AddUpgrades (Variables|/Script/Wipgate.RTS_PlayerController|GetTeam _asrts_player_controller) (Variables|Default|GetUpgradesArr))
      (CallFunction|LogUpgrades)
      (Audio|PlaySoundatLocation "/Game/Art/Sounds/Shop/ShopPurchase2_Cue.ShopPurchase2_Cue" (Transformation|GetActorLocation) "0, 0, 0" 1.0 1.0 0.0 "/Game/Art/Sounds/SA_EffectSounds.SA_EffectSounds" "/Game/Art/Sounds/SCo_EffectSounds.SCo_EffectSounds")
      (Actor|DestroyActor)
      (Utilities|Array|RemoveItem (Variables|/Game/Code/PowerUps/BP_UpgradeShop.BP_UpgradeShop_C|GetShopItems (Variables|Default|GetUpgrade%20Shop)) self))))

(fn ConstructionScript
  (|CallParentFunction)
  (bind _cost_string (CallFunction|GetCostString))
  (Rendering|Components|TextRender|SetText (Variables|Default|GetTextRender) (Utilities|Text|ToText(String) _cost_string)))

(fn GetCostString
  (return (Utilities|String|Append (Utilities|String|ToString(Integer) (Variables|Default|GetCost)) " Luma")))

(fn SetHidden
  (params (inputIsHidden :type Boolean))
  (bind _output_get (Variables|Default|SetHidden inputIsHidden))
  (Rendering|SetActorHiddenInGame _output_get)
  (if _output_get
    (Variables|Default|SetHovering false)
    (Rendering|SetVisibility (Variables|Default|GetScreen%20UI) false true)
    (Variables|Default|SetHover%20Time 0.0)))