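; World pickup actor for a purchasable power-up, shown as a bobbing, spinning icon with colored light, sphere and name/price text.
; Hovering briefly reveals a screen-space info popup, and clicking starts a timed spin-up and pulsing shrink.
; It then spawns price-scaled particles, adds its upgrades to the player team via RTS_GameState entities, and destroys itself.
; Price deduction and obtained-list tracking are only debug prints.
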(event OnBeginCursorOver(Sphere)
  (params (TouchedComponent :type Primitive%20Component%20Object%20Reference))
  (Variables|Default|SetHovering true))

(event OnEndCursorOver(Sphere)
  (params (TouchedComponent :type Primitive%20Component%20Object%20Reference))
  (bind _output_get (Variables|Default|SetHovering false))
  (Rendering|SetVisibility (Variables|Default|GetScreenUI) _output_get true)
  (Variables|Default|SetHoverTime 0.0))

(event OnClicked(Sphere)
  (params (TouchedComponent :type Primitive%20Component%20Object%20Reference) (ButtonPressed :type Key%20Structure))
  (Variables|Default|SetIsDisappearing true))

(event EventBeginPlay
  (bind _asui_power_up_pop_up_info (Utilities|Casting|CastToUI_PowerUpPopUpInfo (UserInterface|GetUserWidgetObject (Variables|Default|GetScreenUI))))
  (Default|SetVariables _asui_power_up_pop_up_info (Utilities|Text|ToText(String) (Variables|Default|GetName)) (Utilities|Text|ToText(String) (Variables|Default|GetDescription)) (Variables|Default|GetCardIcon)))

(event Collision|EventActorBeginOverlap
  (params (OtherActor :type Actor%20Object%20Reference)))

(event EventTick
  (params (DeltaSeconds :type Float%20%28single-precision%29))
  (Transformation|SetRelativeLocation (Variables|Default|GetPointLight) (Math|Vector|MakeVector 0.0 0.0 (+ (Variables|Default|GetFloatHeight) (* (Math|Trig|Sin(Radians) (* (Actor|GetGameTimeSinceCreation) (Variables|Default|GetFloatSpeed))) (Variables|Default|GetFloatDistance)))) false false)
  (Transformation|SetWorldRotation (Variables|Default|GetIcon) (Math|Rotator|MakeRotator 0.0 0.0 (* (Actor|GetGameTimeSinceCreation) (Variables|Default|GetRotationSpeed))) false false)
  (CallFunction|UITick)
  (if (Variables|Default|GetIsDisappearing)
    (CallFunction|Disappear)))

(fn ConstructionScript
  (Components|StaticMesh|SetStaticMesh (Variables|Default|GetIcon) (Variables|Default|GetMesh))
  (Rendering|Material|SetMaterial (Variables|Default|GetIcon) 0 (Variables|Default|GetMeshMaterial))
  (Rendering|Components|Light|SetLightColor (Variables|Default|GetPointLight) (Variables|Default|GetColor) true)
  (bind _returnvalue (Rendering|Material|CreateDynamicMaterialInstance (Variables|Default|GetSphere) 0 (Variables|Default|GetSphereMat) :!class /Script/Engine.PrimitiveComponent))
  (Rendering|Material|SetVectorParameterValue _returnvalue "Color" (Variables|Default|GetColor) :!class /Script/Engine.MaterialInstanceDynamic)
  (Rendering|Components|TextRender|SetText (Variables|Default|GetTextRender) (Utilities|Text|ToText(String) (Utilities|String|Append (Variables|Default|GetName) " 
" (Utilities|String|ToString(Integer) (Variables|Default|GetPrice)) " Luma"))))

(fn UITick
  (if (Variables|Default|GetHovering)
    (bind _output_get (Variables|Default|SetHoverTime (+ (Variables|Default|GetHoverTime) (Utilities|Time|GetWorldDeltaSeconds))))
    (Math|Float|CompareFloat _output_get 0.15
      (:>
        (Rendering|SetVisibility (Variables|Default|GetScreenUI) true true)))))

(fn GetPrice
  (return (Variables|Default|GetPrice)))

(fn Disappear
  (Variables|Default|SetDisappearanceTimer (+ (Variables|Default|GetDisappearanceTimer) (Utilities|Time|GetWorldDeltaSeconds)))
  ;[1 1 1] Rotation
  (Variables|Default|SetRotationSpeed (+ (Variables|Default|GetRotationSpeed) (* (Utilities|Time|GetWorldDeltaSeconds) 1e+02)))
  (Transformation|SetRelativeScale3D (Variables|Default|GetIcon) (Math|Conversions|ToVector(Float) (Math|Float|Clamp(Float) (- (- 1.0 (/ (Math|Trig|Sin(Degrees) (* (+ (* (Variables|Default|GetDisappearanceTimer) 3.0) 0.5) 1.8e+02)) 4.0)) (/ (Variables|Default|GetDisappearanceTimer) (Variables|Default|GetDisappearanceDuration))))))
  ;[1 1 1] Destroy
  (Math|Float|CompareFloat (Variables|Default|GetDisappearanceTimer) (Variables|Default|GetDisappearanceDuration)
    (:>
      (Rendering|SetVisibility (Variables|Default|GetPointLight) false true)
      (bind _returnvalue (Effects|SpawnEmitteratLocation "/Game/Art/ParticleEffects/Pickup/PE_PickUp.PE_PickUp" (Transformation|GetWorldLocation (Variables|Default|GetSphere))))
      (Effects|Components|ParticleSystem|SetFloatParameter _returnvalue "SpawnRate" (Math|Conversions|ToFloat(Integer) (/ (Variables|Default|GetPrice) 10)))
      (Development|PrintString (Utilities|String|Append "Subtract " (Utilities|String|ToString(Integer) (Variables|Default|GetPrice)) " coins from player.") true true "(R=1.000000,G=0.480801,B=0.000000,A=1.000000)")
      (Development|PrintString (Utilities|String|Append "Add \"" (Variables|Default|GetName) "\" to obtained powerups.") true true "(R=1.000000,G=0.000000,B=0.783689,A=1.000000)")
      (CallFunction|AddUpgrades)
      (Actor|DestroyActor))))

(fn AddUpgrades
  (for _array_element (Variables|Gameplay|GetUpgardesArr)
    (LocalVariables|SetLocalUpgrade _array_element)
    (Variables|Gameplay|SetHackyLoopBreak false)
    (bind _asrts_game_state (Utilities|Casting|CastToRTS_GameState (Game|GetGameState)))
    (for _array_element_2 (Variables|/Script/Wipgate.RTS_GameState|GetEntities _asrts_game_state)
      (if (not (Variables|Gameplay|GetHackyLoopBreak))
        (if (Utilities|Enum|Equal(Enum) (Variables|/Script/Wipgate.RTS_Team|GetAlignment (Variables|/Script/Wipgate.RTS_Entity|GetTeam _array_element_2)) "E_PLAYER")
          (Variables|Gameplay|SetHackyLoopBreak true)
          (Class|RTSTeam|AddUpgrade (Variables|/Script/Wipgate.RTS_Entity|GetTeam _array_element_2) (Utilities|Struct|MakeHOTRELOADED_Upgrade_0 (.effect (LocalVariables|GetLocalUpgrade)) (.type (LocalVariables|GetLocalUpgrade)) (.stat (LocalVariables|GetLocalUpgrade))))
          (Development|PrintString (Utilities|String|Append (Utilities|String|ToString(Float) (.effect (LocalVariables|GetLocalUpgrade))) " | " (Utilities|String|EnumtoString (.type (LocalVariables|GetLocalUpgrade))) " | " (Utilities|String|EnumtoString (.stat (LocalVariables|GetLocalUpgrade))) " Added.")))))))