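; Pickup actor that grants the player health or Luma when a player-aligned RTS unit overlaps its collision mesh.
; The overlap routes the amount by pickup type to the player controller; the Effect type only prints a not-implemented message.
; It then plays a death particle and sound at the sphere and destroys itself.
; Tick spins the sphere on combined local and world rotations for a tumbling look.
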(event Custom|OnSphereOverlap
  (params (OverlappedComponent :type Primitive%20Component%20Object%20Reference) (OtherActor :type Actor%20Object%20Reference) (OtherComp :type Primitive%20Component%20Object%20Reference) (OtherBodyIndex :type Integer) (bFromSweep :type Boolean) (SweepResult :type Hit%20Result%20Structure%20%28by%20ref%29))
  (bind _amount (Variables|Pickup|GetAmount))
  (bind _sphere (Variables|Default|GetSphere))
  (bind _returnvalue (Transformation|GetWorldLocation _sphere))
  (bind _asrts_unit (Utilities|Casting|CastToRTS_Unit OtherActor))
  (if (Utilities|Enum|Equal(Enum) (Variables|/Script/Wipgate.RTS_Entity|GetAlignment _asrts_unit) "E_PLAYER")
    (bind _asrts_player_controller (Utilities|Casting|CastToRTS_PlayerController (Game|GetPlayerController 0)))
    (switch Utilities|FlowControl|Switch|SwitchonEnum_PickupType (Variables|Pickup|GetType)
      (:NewEnumerator0
        (Class|RTSPlayerController|AddHealth _asrts_player_controller _amount))
      (:NewEnumerator1
        (Class|RTSPlayerController|AddLuma _asrts_player_controller _amount true))
      (:NewEnumerator2
        (Development|PrintString "EffectType not implemented on pickups")))
    (Effects|SpawnEmitteratLocation "/Game/Art/ParticleEffects/Death/PE_Death.PE_Death" _returnvalue)
    (Audio|PlaySoundatLocation "/Game/Art/Sounds/GameplayFeedback/SW_PickUp_Cue.SW_PickUp_Cue" _returnvalue "0, 0, 0" 1.0 1.0 0.0 "/Game/Art/Sounds/SA_EffectSounds.SA_EffectSounds" "/Game/Art/Sounds/SCo_EffectSounds.SCo_EffectSounds")
    (Actor|DestroyActor)))

(event EventTick
  (params (DeltaSeconds :type Float%20%28single-precision%29))
  (Transformation|AddLocalRotation (Variables|Default|GetSphere) (* "0,-60.000000, 0" DeltaSeconds) false false)
  (Transformation|AddWorldRotation (Variables|Default|GetSphere) (* "0,40.000000, 0" DeltaSeconds) false false))

(event EventBeginPlay
  (|CallParentFunction)
  (Collision|AssignOnComponentBeginOverlap (Variables|Default|GetCollisionMesh) (delegate Custom|OnSphereOverlap)))

(fn ConstructionScript
  (Variables|Default|SetSphereMat (Rendering|Material|GetMaterial (Variables|Default|GetSphere) 0))
  (|CallParentFunction))