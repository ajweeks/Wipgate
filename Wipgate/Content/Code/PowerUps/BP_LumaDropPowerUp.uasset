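; BP_LumaDropPowerUp is a pickup that grants Luma to the player when one of their units touches it.
; On BeginPlay it binds its sphere's begin-overlap event.
; An overlapping RTS unit on the player team makes it add LumaAmount through the RTS player controller, then the pickup destroys itself.
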(event Custom|OnSphereOverlap
  (params (OverlappedComponent :type Primitive%20Component%20Object%20Reference) (OtherActor :type Actor%20Object%20Reference) (OtherComp :type Primitive%20Component%20Object%20Reference) (OtherBodyIndex :type Integer) (bFromSweep :type Boolean) (SweepResult :type Hit%20Result%20Structure%20%28by%20ref%29))
  (bind _asrts_unit (Utilities|Casting|CastToRTS_Unit OtherActor))
  (if (Utilities|Enum|Equal(Enum) (Variables|/Script/Wipgate.RTS_Team|GetAlignment (Variables|/Script/Wipgate.RTS_Entity|GetTeam _asrts_unit)) "E_PLAYER")
    (bind _asrts_player_controller (Utilities|Casting|CastToRTS_PlayerController (Game|GetPlayerController 0)))
    (Class|RTSPlayerController|AddLuma _asrts_player_controller (Variables|Default|GetLuma%20Amount))
    (Actor|DestroyActor)))

(event EventBeginPlay
  (|CallParentFunction)
  (Collision|AssignOnComponentBeginOverlap (Variables|Default|GetSphere) (delegate Custom|OnSphereOverlap)))

(fn ConstructionScript
  (|CallParentFunction))