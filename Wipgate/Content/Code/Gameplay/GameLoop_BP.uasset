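; GameLoop_BP runs the level loop for an RTS, carrying currency and Luma between levels through the game instance.
; On BeginPlay it keeps one random LevelGoal as the end zone, destroys the others and adds the saved amounts to the player controller.
; ContinueToNextLevel saves both currencies and reopens the current level.
; The upgrade re-application branch is disconnected and SaveUnits is empty.
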(event EventBeginPlay
  ;[1 1 1] Get game instance
  (bind _asrts_game_instance_bp (Utilities|Casting|CastToRTS_GameInstance_BP (Game|GetGameInstance))
    (:then
      (Variables|Default|SetGameInstance _asrts_game_instance_bp))
    (:CastFailed
      (Development|PrintString "Cast to RTS_GameInstance_BP failed")))
  ;[1 1 1] Get potential end zones and pick one
  (bind _outactors (Actor|GetAllActorsOfClass "/Game/Code/Gameplay/LevelGoal.LevelGoal_C"))
  (bind _output_get (Variables|Default|SetPotentialEndZones _outactors))
  (Variables|Default|SetEndZone (Utilities|Array|Get(acopy) _output_get (Math|Random|RandomInteger (Utilities|Array|Length _output_get))))
  (for _array_element (Variables|Default|GetPotentialEndZones)
    (if (!= _array_element (Variables|Default|GetEndZone))
      (Actor|DestroyActor _array_element)))
  (bind _asrts_player_controller_bp (Utilities|Casting|CastToRTS_PlayerController_BP (Game|GetPlayerController 0)))
  (Class|RTSPlayerController|AddCurrency _asrts_player_controller_bp (Variables|/Script/Wipgate.RTS_GameInstance|GetCurrentCurrency (Variables|Default|GetGameInstance)))
  (Class|RTSPlayerController|AddLuma _asrts_player_controller_bp (Variables|/Script/Wipgate.RTS_GameInstance|GetCurrentLuma (Variables|Default|GetGameInstance))))

(event Collision|EventActorBeginOverlap
  (params (OtherActor :type Actor%20Object%20Reference)))

(event EventTick
  (params (DeltaSeconds :type Float%20%28single-precision%29)))

(fn ConstructionScript)

(fn ContinuetoNextLevel
  (bind _asrts_player_controller_bp (Utilities|Casting|CastToRTS_PlayerController_BP (Game|GetPlayerController 0)))
  (Variables|Default|SetPlayerController _asrts_player_controller_bp)
  (CallFunction|SaveCurrency)
  (bind _returnvalue (Game|GetCurrentLevelName true))
  (Game|OpenLevel(byName) (Utilities|String|StringToName _returnvalue)))

(fn SaveCurrency
  ;[1 1 1] Save currencies
  (bind _returnvalue (Class|RTSPlayerController|GetCurrentCurrencyAmount (Variables|Default|GetPlayerController)))
  (Variables|/Script/Wipgate.RTS_GameInstance|SetCurrentCurrency (Variables|Default|GetGameInstance) _returnvalue)
  (bind _returnvalue_2 (Class|RTSPlayerController|GetCurrentLumaAmount (Variables|Default|GetPlayerController)))
  (Variables|/Script/Wipgate.RTS_GameInstance|SetCurrentLuma (Variables|Default|GetGameInstance) _returnvalue_2))

(fn SaveUnits)