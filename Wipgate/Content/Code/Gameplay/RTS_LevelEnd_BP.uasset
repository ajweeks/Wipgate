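; Level goal zone for an RTS that ends the round once enough friendly units reach it.
; Its collision box flags units as in the goal; completion requires no enemies in the end zone and no spawned entities left on an optional spawner.
; Goal entry or any unit death checks the friendly percentage, then after a short delay ends the round and shows the end screen.
; Tick recolors the mesh green or red by completability.
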(event OnComponentBeginOverlap(CollisionBox)
  (params (OverlappedComponent :type Primitive%20Component%20Object%20Reference) (OtherActor :type Actor%20Object%20Reference) (OtherComp :type Primitive%20Component%20Object%20Reference) (OtherBodyIndex :type Integer) (bFromSweep :type Boolean) (SweepResult :type Hit%20Result%20Structure%20%28by%20ref%29))
  (bind _asrts_unit (Utilities|Casting|CastToRTS_Unit OtherActor))
  (Variables|/Script/Wipgate.RTS_Unit|SetInLevelGoal _asrts_unit true)
  (if (Variables|Default|GetCan%20Be%20Completed)
    (bind _asrts_game_state (Utilities|Casting|CastToRTS_GameState (Game|GetGameState)))
    (bind _returnvalue (Class|RTSGameState|GetPercentOfFriendlyUnitsinLevelGoal _asrts_game_state))
    (if (>= _returnvalue (Variables|Default|GetPercent%20Of%20Units%20Required%20for%20Completion))
      (Utilities|FlowControl|Delay 1.0)
      (if (not (Variables|Default|GetHas%20Been%20Completed))
        (Variables|Default|SetHas%20Been%20Completed true)
        (Development|PrintString "Level complete." true true "(R=0.022114,G=1.000000,B=0.000000,A=1.000000)")
        (bind _asrts_game_instance (Utilities|Casting|CastToRTS_GameInstance (Game|GetGameInstance)))
        (Class|RTSGameInstance|EndRound _asrts_game_instance)
        (bind _asrts_player_controller_bp (Utilities|Casting|CastToRTS_PlayerController_BP (Game|GetPlayerController 0)))
        (bind _returnvalue_2 (Class|RTSPlayerController|GetRTSHUDBase _asrts_player_controller_bp))
        (bind _asrts_hud_bp (Utilities|Casting|CastToRTS_HUD_BP _returnvalue_2))
        (Default|ShowEndScreen _asrts_hud_bp)))))

(event OnComponentEndOverlap(CollisionBox)
  (params (OverlappedComponent :type Primitive%20Component%20Object%20Reference) (OtherActor :type Actor%20Object%20Reference) (OtherComp :type Primitive%20Component%20Object%20Reference) (OtherBodyIndex :type Integer))
  (bind _asrts_unit (Utilities|Casting|CastToRTS_Unit OtherActor))
  (Variables|/Script/Wipgate.RTS_Unit|SetInLevelGoal _asrts_unit false))

(event Custom|OnUnitDeath
  (params (entity :type RTS%20Entity%20Object%20Reference))
  (CallFunction|UpdateCanbeCompleted)
  (if (Variables|Default|GetCan%20Be%20Completed)
    (bind _asrts_game_state (Utilities|Casting|CastToRTS_GameState (Game|GetGameState)))
    (bind _returnvalue (Class|RTSGameState|GetPercentOfFriendlyUnitsinLevelGoal _asrts_game_state))
    (if (>= _returnvalue (Variables|Default|GetPercent%20Of%20Units%20Required%20for%20Completion))
      (Utilities|FlowControl|Delay 1.0)
      (if (not (Variables|Default|GetHas%20Been%20Completed))
        (Variables|Default|SetHas%20Been%20Completed true)
        (Development|PrintString "Level complete." true true "(R=0.022114,G=1.000000,B=0.000000,A=1.000000)")
        (bind _asrts_game_instance (Utilities|Casting|CastToRTS_GameInstance (Game|GetGameInstance)))
        (Class|RTSGameInstance|EndRound _asrts_game_instance)
        (bind _asrts_player_controller_bp (Utilities|Casting|CastToRTS_PlayerController_BP (Game|GetPlayerController 0)))
        (bind _returnvalue_2 (Class|RTSPlayerController|GetRTSHUDBase _asrts_player_controller_bp))
        (bind _asrts_hud_bp (Utilities|Casting|CastToRTS_HUD_BP _returnvalue_2))
        (Default|ShowEndScreen _asrts_hud_bp)))))

(event EventTick
  (params (DeltaSeconds :type Float%20%28single-precision%29))
  (bind _staticmesh (Variables|Default|GetStaticMesh))
  (bind _returnvalue (Rendering|Material|GetMaterial _staticmesh 0))
  (bind _can_be_completed (CallFunction|UpdateCanbeCompleted))
  (if _can_be_completed
    (bind _returnvalue_2 (Rendering|Material|CreateDynamicMaterialInstance _staticmesh 0 _returnvalue :!class /Script/Engine.PrimitiveComponent))
    (Rendering|Material|SetVectorParameterValue _returnvalue_2 "Color" "(R=0.035794,G=1.000000,B=0.000000,A=1.000000)" :!class /Script/Engine.MaterialInstanceDynamic)
    (else
      (bind _returnvalue_3 (Rendering|Material|CreateDynamicMaterialInstance _staticmesh 0 _returnvalue :!class /Script/Engine.PrimitiveComponent))
      (Rendering|Material|SetVectorParameterValue _returnvalue_3 "Color" "(R=1.000000,G=0.017360,B=0.000000,A=1.000000)" :!class /Script/Engine.MaterialInstanceDynamic))))

(event EventBeginPlay
  (bind _asrts_game_state_bp (Utilities|Casting|CastToRTS_GameState_BP (Game|GetGameState)))
  (EventDispatchers|BindEventtoOnDeathDelegate _asrts_game_state_bp (delegate Custom|OnUnitDeath))
  (for _array_element (Collision|GetOverlappingActors (Variables|Default|GetCollision%20Box) "/Script/Wipgate.RTS_Unit" :!class /Script/Engine.PrimitiveComponent)
    (bind _asrts_unit (Utilities|Casting|CastToRTS_Unit _array_element))
    (Variables|/Script/Wipgate.RTS_Unit|SetInLevelGoal _asrts_unit true)))

(fn ConstructionScript
  (Transformation|SetWorldScale3D (Variables|Default|GetMinimapIcon) "15.000000,15.000000,15.000000"))

(fn UpdateCanbeCompleted
  (bind _asrts_entity_spawner_bp (Utilities|Casting|CastToRTS_EntitySpawner_BP (Variables|Default|GetEntitySpawner))
    (:then
      (bind _returnvalue (Class|RTSGameState|AreEnemiesinEndZone (.AsRTS%20Game%20State%20BP (Utilities|Casting|CastToRTS_GameState_BP (Game|GetGameState)))))
      (bind _output_get (Variables|Default|SetCan%20Be%20Completed (not (or _returnvalue (> (Utilities|Array|Length (Variables|/Script/Wipgate.RTS_EntitySpawnerBase|Getm_SpawnedEntities _asrts_entity_spawner_bp)) 0)))))
      (return _output_get))
    (:CastFailed
      (bind _returnvalue_2 (Class|RTSGameState|AreEnemiesinEndZone (.AsRTS%20Game%20State%20BP (Utilities|Casting|CastToRTS_GameState_BP (Game|GetGameState)))))
      (bind _output_get_2 (Variables|Default|SetCan%20Be%20Completed (not _returnvalue_2)))
      (return _output_get_2))))