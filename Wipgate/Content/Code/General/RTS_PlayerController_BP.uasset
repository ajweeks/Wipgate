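; RTS player controller that turns player input into unit orders and ability use, and handles pause and UI toggles.
; BeginPlay spawns the movement and Luma ability actors, links them to HUD icons and creates a custom cursor.
; Clicks send move, attack or attack-move commands to selected units' AI controllers, using square-grid formations for ground targets.
; Ability selection checks cooldowns, fires self-cast abilities immediately, and updates icon animations and cursor textures.
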(event EventOnAbilitySpecialistActiveActivate
  ;[1 1 1] Specialist Abilities
  (bind _returnvalue (Class|RTSPlayerController|GetRTSHUDBase))
  (bind _asrts_hud_bp (Utilities|Casting|CastToRTS_HUD_BP _returnvalue))
  (if (Widget|IsVisible (Variables|/Game/Code/User_Interface/RTS_HUD_BP.RTS_HUD_BP_C|GetSpecialistAbilityButtonHolder _asrts_hud_bp))
    (Default|OnActivated (Variables|/Game/Code/User_Interface/RTS_HUD_BP.RTS_HUD_BP_C|GetSpecialistAbilityActiveIcon _asrts_hud_bp))))

(event EventOnAbilitySpecialistConstructActivate
  ;[1 1 1] Specialist Abilities
  (bind _returnvalue (Class|RTSPlayerController|GetRTSHUDBase))
  (bind _asrts_hud_bp (Utilities|Casting|CastToRTS_HUD_BP _returnvalue))
  (if (Widget|IsVisible (Variables|/Game/Code/User_Interface/RTS_HUD_BP.RTS_HUD_BP_C|GetSpecialistAbilityButtonHolder _asrts_hud_bp))
    (Default|OnActivated (Variables|/Game/Code/User_Interface/RTS_HUD_BP.RTS_HUD_BP_C|GetSpecialistAbilityConstructIcon _asrts_hud_bp))))

(event EventOnAbilitySpecialistActiveSelect
  ;[1 1 1] Specialist Abilities
  (bind (_specialist _success) (CallFunction|GetSpecialistSelected))
  (if _success
    (bind (_selected _activated) (CallFunction|OnAbilitySelected (Variables|/Script/Wipgate.RTS_Specialist|GetAbilityActive _specialist)))
    (bind _returnvalue (Class|RTSPlayerController|GetRTSHUDBase))
    (bind _asrts_hud_bp (Utilities|Casting|CastToRTS_HUD_BP _returnvalue))
    (CallFunction|PlayAbilityIconAnim (Variables|/Game/Code/User_Interface/RTS_HUD_BP.RTS_HUD_BP_C|GetSpecialistAbilityActiveIcon _asrts_hud_bp) _selected _activated)
    (if _selected
      (Class|RTSCursor|SetCursorTexture (Variables|Default|GetCursorRef) (Variables|/Script/Wipgate.Ability|GetCursorIconTexture (Variables|/Script/Wipgate.RTS_Specialist|GetAbilityActive _specialist))))))

(event EventOnAbilitySpecialistConstructSelect
  ;[1 1 1] Specialist Abilities
  (bind (_specialist _success) (CallFunction|GetSpecialistSelected))
  (if _success
    (bind (_selected _activated) (CallFunction|OnAbilitySelected (Variables|/Script/Wipgate.RTS_Specialist|GetAbilityConstruct _specialist)))
    (bind _returnvalue (Class|RTSPlayerController|GetRTSHUDBase))
    (bind _asrts_hud_bp (Utilities|Casting|CastToRTS_HUD_BP _returnvalue))
    (CallFunction|PlayAbilityIconAnim (Variables|/Game/Code/User_Interface/RTS_HUD_BP.RTS_HUD_BP_C|GetSpecialistAbilityConstructIcon _asrts_hud_bp) _selected _activated)
    (if _selected
      (Class|RTSCursor|SetCursorTexture (Variables|Default|GetCursorRef) (Variables|/Script/Wipgate.Ability|GetCursorIconTexture (Variables|/Script/Wipgate.RTS_Specialist|GetAbilityConstruct _specialist))))))

(event EventOnAbilitySpecialistPassiveActivate
  ;[1 1 1] Specialist Abilities
  (bind _returnvalue (Class|RTSPlayerController|GetRTSHUDBase))
  (bind _asrts_hud_bp (Utilities|Casting|CastToRTS_HUD_BP _returnvalue))
  (if (Widget|IsVisible (Variables|/Game/Code/User_Interface/RTS_HUD_BP.RTS_HUD_BP_C|GetSpecialistAbilityButtonHolder _asrts_hud_bp))
    (Default|OnActivated (Variables|/Game/Code/User_Interface/RTS_HUD_BP.RTS_HUD_BP_C|GetSpecialistAbilityPassiveIcon _asrts_hud_bp))))

(event EventOnAbilitySpecialistPassiveSelect
  ;[1 1 1] Specialist Abilities
  (bind (_specialist _success) (CallFunction|GetSpecialistSelected))
  (if _success
    (bind (_selected _activated) (CallFunction|OnAbilitySelected (Variables|/Script/Wipgate.RTS_Specialist|GetAbilityPassive _specialist)))
    (bind _returnvalue (Class|RTSPlayerController|GetRTSHUDBase))
    (bind _asrts_hud_bp (Utilities|Casting|CastToRTS_HUD_BP _returnvalue))
    (CallFunction|PlayAbilityIconAnim (Variables|/Game/Code/User_Interface/RTS_HUD_BP.RTS_HUD_BP_C|GetSpecialistAbilityPassiveIcon _asrts_hud_bp) _selected _activated)
    (if _selected
      (Class|RTSCursor|SetCursorTexture (Variables|Default|GetCursorRef) (Variables|/Script/Wipgate.Ability|GetCursorIconTexture (Variables|/Script/Wipgate.RTS_Specialist|GetAbilityPassive _specialist))))))

(event EventOnAbilityMovementMoveActivate
  (bind _returnvalue (Game|Player|IsInputKeyDown "LeftShift"))
  ;[1 1 1] Movement Abilities
  (bind _returnvalue_2 (Class|RTSPlayerController|GetRTSHUDBase))
  (bind _asrts_hud_bp (Utilities|Casting|CastToRTS_HUD_BP _returnvalue_2))
  (if (Widget|IsVisible (Variables|/Game/Code/User_Interface/RTS_HUD_BP.RTS_HUD_BP_C|GetMovementAbilityButtonHolder _asrts_hud_bp))
    (bind _asrts_aicontroller (Utilities|Casting|CastToRTS_AIController (AI|GetAIController 0)))
    (bind _asrts_game_state_bp (Utilities|Casting|CastToRTS_GameState_BP (Game|GetGameState)))
    (if (== (Utilities|Array|Length (Variables|/Script/Wipgate.RTS_GameState|GetSelectedEntities _asrts_game_state_bp)) 1)
      (Class|RTSAIController|AddCommandMovetoEntity _asrts_aicontroller (Utilities|Array|Get(acopy) (Variables|/Script/Wipgate.RTS_GameState|GetSelectedEntities _asrts_game_state_bp)) false _returnvalue)
      (else
        (bind _mouse_pos_world_space (CallFunction|GetMousePosGround))
        (Class|RTSAIController|AddCommandMovetoLocation _asrts_aicontroller _mouse_pos_world_space false _returnvalue)))))

(event EventOnAbilityMovementAttackMoveActivate
  ;[1 1 1] Movement Abilities
  (bind _returnvalue (Class|RTSPlayerController|GetRTSHUDBase))
  (bind _asrts_hud_bp (Utilities|Casting|CastToRTS_HUD_BP _returnvalue))
  (if (Widget|IsVisible (Variables|/Game/Code/User_Interface/RTS_HUD_BP.RTS_HUD_BP_C|GetMovementAbilityButtonHolder _asrts_hud_bp))
    (bind _asrts_aicontroller (Utilities|Casting|CastToRTS_AIController (AI|GetAIController 0)))
    (bind _mouse_pos_world_space (CallFunction|GetMousePosGround))
    (Class|RTSAIController|AddCommandAttackMove _asrts_aicontroller _mouse_pos_world_space false (Game|Player|IsInputKeyDown "LeftShift"))))

(event EventOnAbilityMovementStopSelect
  (bind _cursorref (Variables|Default|GetCursorRef))
  ;[1 1 1] Movement Abilities
  (bind _returnvalue (Class|RTSPlayerController|GetRTSHUDBase))
  (bind _asrts_hud_bp (Utilities|Casting|CastToRTS_HUD_BP _returnvalue))
  (if (Widget|IsVisible (Variables|/Game/Code/User_Interface/RTS_HUD_BP.RTS_HUD_BP_C|GetMovementAbilityButtonHolder _asrts_hud_bp))
    (bind (_selected _activated) (CallFunction|OnAbilitySelected (Variables|Default|GetAbilityMovementStop)))
    (CallFunction|PlayAbilityIconAnim (Variables|/Game/Code/User_Interface/RTS_HUD_BP.RTS_HUD_BP_C|GetMovementAbilityStopIcon _asrts_hud_bp) _selected _activated)
    (if _selected
      (Class|RTSCursor|SetCursorTexture _cursorref (Variables|/Script/Wipgate.RTS_Cursor|GetStopCircleTexture _cursorref)))))

(event EventUpdateSelectedEntities
  (params (SelectedEntities :type Array%20of%20RTS%20Entity%20Object%20References))
  ;[1 1 1] Update Selected Entities
  (if (== (Utilities|Array|Length SelectedEntities) 0)
    (if (Utilities|IsValid (Variables|Default|GetSelected%20Icon))
      (Default|ResetAnimation (Variables|Default|GetSelected%20Icon)))
    (Variables|Default|SetSelected%20Icon 0)))

(event EventOnAbilityMovementMoveSelect
  (bind _cursorref (Variables|Default|GetCursorRef))
  ;[1 1 1] Movement Abilities
  (bind _returnvalue (Class|RTSPlayerController|GetRTSHUDBase))
  (bind _asrts_hud_bp (Utilities|Casting|CastToRTS_HUD_BP _returnvalue))
  (if (Widget|IsVisible (Variables|/Game/Code/User_Interface/RTS_HUD_BP.RTS_HUD_BP_C|GetMovementAbilityButtonHolder _asrts_hud_bp))
    (bind (_selected _activated) (CallFunction|OnAbilitySelected (Variables|Default|GetAbilityMovementMove)))
    (CallFunction|PlayAbilityIconAnim (Variables|/Game/Code/User_Interface/RTS_HUD_BP.RTS_HUD_BP_C|GetMovementAbilityMoveIcon _asrts_hud_bp) _selected _activated)
    (if _selected
      (Class|RTSCursor|SetCursorTexture _cursorref (Variables|/Script/Wipgate.RTS_Cursor|GetMoveTexture _cursorref)))))

(event EventOnAbilityMovementStopActivate
  ;[1 1 1] Movement Abilities
  (bind _returnvalue (Class|RTSPlayerController|GetRTSHUDBase))
  (bind _asrts_hud_bp (Utilities|Casting|CastToRTS_HUD_BP _returnvalue))
  (if (Widget|IsVisible (Variables|/Game/Code/User_Interface/RTS_HUD_BP.RTS_HUD_BP_C|GetMovementAbilityButtonHolder _asrts_hud_bp))
    (bind _asrts_aicontroller (Utilities|Casting|CastToRTS_AIController (AI|GetAIController 0)))
    (Class|RTSAIController|AddCommandStop _asrts_aicontroller)))

(event EventOnAbilityMovementHoldPositionSelect
  (bind _cursorref (Variables|Default|GetCursorRef))
  ;[1 1 1] Movement Abilities
  (bind _returnvalue (Class|RTSPlayerController|GetRTSHUDBase))
  (bind _asrts_hud_bp (Utilities|Casting|CastToRTS_HUD_BP _returnvalue))
  (if (Widget|IsVisible (Variables|/Game/Code/User_Interface/RTS_HUD_BP.RTS_HUD_BP_C|GetMovementAbilityButtonHolder _asrts_hud_bp))
    (bind (_selected _activated) (CallFunction|OnAbilitySelected (Variables|Default|GetAbilityMovementHoldPosition)))
    (CallFunction|PlayAbilityIconAnim (Variables|/Game/Code/User_Interface/RTS_HUD_BP.RTS_HUD_BP_C|GetMovementAbilityHoldPositionIcon _asrts_hud_bp) _selected _activated)
    (if _selected
      (Class|RTSCursor|SetCursorTexture _cursorref (Variables|/Script/Wipgate.RTS_Cursor|GetStopCircleTexture _cursorref)))))

(event EventOnAbilityMovementAttackMoveSelect
  (bind _cursorref (Variables|Default|GetCursorRef))
  ;[1 1 1] Movement Abilities
  (bind _returnvalue (Class|RTSPlayerController|GetRTSHUDBase))
  (bind _asrts_hud_bp (Utilities|Casting|CastToRTS_HUD_BP _returnvalue))
  (if (Widget|IsVisible (Variables|/Game/Code/User_Interface/RTS_HUD_BP.RTS_HUD_BP_C|GetMovementAbilityButtonHolder _asrts_hud_bp))
    (bind (_selected _activated) (CallFunction|OnAbilitySelected (Variables|Default|GetAbilityMovementAttackMove)))
    (CallFunction|PlayAbilityIconAnim (Variables|/Game/Code/User_Interface/RTS_HUD_BP.RTS_HUD_BP_C|GetMovementAbilityAttackMoveIcon _asrts_hud_bp) _selected _activated)
    (if _selected
      (Class|RTSCursor|SetCursorTexture _cursorref (Variables|/Script/Wipgate.RTS_Cursor|GetAttackMoveTexture _cursorref)))))

(event EventOnAbilityMovementHoldPositionActivate
  ;[1 1 1] Movement Abilities
  (bind _returnvalue (Class|RTSPlayerController|GetRTSHUDBase))
  (bind _asrts_hud_bp (Utilities|Casting|CastToRTS_HUD_BP _returnvalue))
  (if (Widget|IsVisible (Variables|/Game/Code/User_Interface/RTS_HUD_BP.RTS_HUD_BP_C|GetMovementAbilityButtonHolder _asrts_hud_bp))
    (bind _asrts_aicontroller (Utilities|Casting|CastToRTS_AIController (AI|GetAIController 0)))
    (bind _mouse_pos_world_space (CallFunction|GetMousePosGround))
    (Class|RTSAIController|AddCommandAttackMove _asrts_aicontroller _mouse_pos_world_space false (Game|Player|IsInputKeyDown "LeftShift"))))

(event EventBeginPlay
  (bind _returnvalue (Transformation|GetActorTransform))
  (bind _abilitymovementmoveclass (Variables|Default|GetAbilityMovementMoveClass))
  (bind _abilitymovementattackmoveclass (Variables|Default|GetAbilityMovementAttackMoveClass))
  (bind _abilitymovementstopclass (Variables|Default|GetAbilityMovementStopClass))
  (bind _abilitymovementholdpositionclass (Variables|Default|GetAbilityMovementHoldPositionClass))
  (bind _abilitylumaapplyclass (Variables|Default|GetAbilityLumaApplyClass))
  ;[1 1 1] Spawn ability actors
  (|CallParentFunction)
  ;;[1 1 1] Required for HUD member to be set correctly
  (Utilities|FlowControl|Delay 0.0)
  (bind _returnvalue_2 (Class|RTSPlayerController|GetRTSHUDBase))
  (bind _asrts_hud_bp (Utilities|Casting|CastToRTS_HUD_BP _returnvalue_2)
    (:then
      (Utilities|FlowControl|Sequence
        (:then_0
          (if (Utilities|IsValidClass _abilitymovementmoveclass)
            (bind _returnvalue_3 (Game|SpawnActorfromClass _abilitymovementmoveclass _returnvalue "Undefined" 0 0))
            (bind _output_get (Variables|Default|SetAbilityMovementMove _returnvalue_3))
            (Variables|/Script/Wipgate.Ability|Setm_Caster _output_get self)
            (Variables|/Script/Wipgate.Ability|SetIcon _output_get (Variables|/Game/Code/User_Interface/RTS_HUD_BP.RTS_HUD_BP_C|GetMovementAbilityMoveIcon _asrts_hud_bp))
            (else
              (Development|PrintString "Ability class not set in player controller!" true true "(R=1.000000,G=0.050881,B=0.000000,A=1.000000)" 1e+02 :!label _label))))
        (:then_1
          (if (Utilities|IsValidClass _abilitymovementattackmoveclass)
            (bind _returnvalue_4 (Game|SpawnActorfromClass _abilitymovementattackmoveclass _returnvalue "Undefined" 0 0))
            (bind _output_get_2 (Variables|Default|SetAbilityMovementAttackMove _returnvalue_4))
            (Variables|/Script/Wipgate.Ability|Setm_Caster _output_get_2 self)
            (Variables|/Script/Wipgate.Ability|SetIcon _output_get_2 (Variables|/Game/Code/User_Interface/RTS_HUD_BP.RTS_HUD_BP_C|GetMovementAbilityAttackMoveIcon _asrts_hud_bp))
            (else
              (goto _label))))
        (:then_2
          (if (Utilities|IsValidClass _abilitymovementstopclass)
            (bind _returnvalue_5 (Game|SpawnActorfromClass _abilitymovementstopclass _returnvalue "Undefined" 0 0))
            (bind _output_get_3 (Variables|Default|SetAbilityMovementStop _returnvalue_5))
            (Variables|/Script/Wipgate.Ability|Setm_Caster _output_get_3 self)
            (Variables|/Script/Wipgate.Ability|SetIcon _output_get_3 (Variables|/Game/Code/User_Interface/RTS_HUD_BP.RTS_HUD_BP_C|GetMovementAbilityStopIcon _asrts_hud_bp))
            (else
              (goto _label))))
        (:then_3
          (if (Utilities|IsValidClass _abilitymovementholdpositionclass)
            (bind _returnvalue_6 (Game|SpawnActorfromClass _abilitymovementholdpositionclass _returnvalue "Undefined" 0 0))
            (bind _output_get_4 (Variables|Default|SetAbilityMovementHoldPosition _returnvalue_6))
            (Variables|/Script/Wipgate.Ability|Setm_Caster _output_get_4 self)
            (Variables|/Script/Wipgate.Ability|SetIcon _output_get_4 (Variables|/Game/Code/User_Interface/RTS_HUD_BP.RTS_HUD_BP_C|GetMovementAbilityHoldPositionIcon _asrts_hud_bp))
            (else
              (goto _label))))
        (:then_4
          (if (Utilities|IsValidClass _abilitylumaapplyclass)
            (bind _returnvalue_7 (Game|SpawnActorfromClass _abilitylumaapplyclass _returnvalue "Undefined" 0 0))
            (bind _output_get_5 (Variables|Default|SetAbilityLumaApply _returnvalue_7))
            (Variables|/Script/Wipgate.Ability|Setm_Caster _output_get_5 self)
            (Variables|/Script/Wipgate.Ability|SetIcon _output_get_5 (Variables|/Game/Code/User_Interface/RTS_HUD_BP.RTS_HUD_BP_C|GetLumaAbilityApplyIcon _asrts_hud_bp))
            (else
              (goto _label))))
        (:then_5
          ;;[1 1 1] Spawn Custom Cursor
          (bind _returnvalue_8 (UserInterface|CreateWidget "/Game/Code/User_Interface/RTS_Cursor_BP.RTS_Cursor_BP_C" self))
          (bind _output_get_6 (Variables|Default|SetCursorRef _returnvalue_8))
          (UserInterface|Viewport|AddtoViewport _output_get_6 0))))
    (:CastFailed
      (Development|PrintString "HUD isn't RTS_HUD_BP!" true true "(R=1.000000,G=0.000000,B=0.000000,A=1.000000)" 1e+02))))

(event EventOnAbilityLumaApplySelect
  ;[1 1 1] Luma Abilities
  (bind _returnvalue (Class|RTSPlayerController|GetRTSHUDBase))
  (bind _asrts_hud_bp (Utilities|Casting|CastToRTS_HUD_BP _returnvalue))
  (if (Widget|IsVisible (Variables|/Game/Code/User_Interface/RTS_HUD_BP.RTS_HUD_BP_C|GetLumaAbilityButtonHolder _asrts_hud_bp))
    (bind _asrts_game_state_bp (Utilities|Casting|CastToRTS_GameState_BP (Game|GetGameState)))
    (if (> (Utilities|Array|Length (Variables|/Script/Wipgate.RTS_GameState|GetSelectedEntities _asrts_game_state_bp)) 0)
      (bind (_selected _activated) (CallFunction|OnAbilitySelected (Variables|Default|GetAbilityLumaApply)))
      (CallFunction|PlayAbilityIconAnim (Variables|/Game/Code/User_Interface/RTS_HUD_BP.RTS_HUD_BP_C|GetLumaAbilityApplyIcon _asrts_hud_bp) _selected _activated))))

(event Input|ActionEvents|InputActionSecondaryClick
  (params (Key :type Key%20Structure))
  (bind _returnvalue (Game|Player|IsInputKeyDown "LeftShift"))
  (bind _returnvalue_2 (Game|GetPlayerController 0))
  (bind _hitresult (Game|Player|GetHitResultUnderCursorbyChannel _returnvalue_2 "TraceTypeQuery2" true))
  (bind (_bblockinghit _binitialoverlap _time _distance _location _impactpoint _normal _impactnormal _physmat _hitactor) (Collision|BreakHitResult _hitresult))
  ;[1 1 1] Right-click movement
  ;;[1 1 1] Get Gamestate on right mouse
  (:Pressed
    (bind _asrts_game_state_bp (Utilities|Casting|CastToRTS_GameState_BP (Game|GetGameState)))
    ;;[1 1 1] Check if user has units selected
    (if (> (Utilities|Array|Length (Variables|/Script/Wipgate.RTS_GameState|GetSelectedEntities _asrts_game_state_bp)) 0)
      ;;[1 1 1] Raycast from mouse
      (bind _asrts_entity (Utilities|Casting|CastToRTS_Entity _hitactor)
        (:then
          (if (Class|RTSEntity|IsAlive _asrts_entity)
            ;;[1 1 1] If selection was character
            (for _array_element (Variables|/Script/Wipgate.RTS_GameState|GetSelectedEntities _asrts_game_state_bp)
              (if (!= _array_element _asrts_entity)
                (bind _asai_unit_controller (Utilities|Casting|CastToAI_UnitController (AI|GetAIController _array_element)))
                (bind _returnvalue_3 (Class|RTSAIController|GetRelativeAlignment _asai_unit_controller (Variables|/Script/Wipgate.RTS_AIController|Getm_Entity _asai_unit_controller) _asrts_entity))
                (if (Utilities|Enum|Equal(Enum) _returnvalue_3 "E_FRIENDLY")
                  (Class|RTSAIController|AddCommandMovetoEntity _asai_unit_controller _asrts_entity true _returnvalue)
                  (else
                    (Class|RTSAIController|AddCommandAttack _asai_unit_controller _asrts_entity true _returnvalue)))))
            (else
              (if (.ReturnValue (AI|Navigation|ProjectPointtoNavigation _location 0 0 "0, 0, 0")) :!label _label
                (bind _newparam (CallFunction|GetSquadFormation _location))
                (Variables|Default|SetSquadFormation _newparam)
                ;;[1 1 1] If selection was non-character
                (for _array_element_2 (Variables|/Script/Wipgate.RTS_GameState|GetSelectedEntities _asrts_game_state_bp)
                  (bind _asai_unit_controller_2 (Utilities|Casting|CastToAI_UnitController (AI|GetAIController _array_element_2)))
                  (Class|RTSAIController|AddCommandMovetoLocation _asai_unit_controller_2 (.Value (Utilities|Map|Find (Variables|Default|GetSquadFormation) _array_element_2)) true (Game|Player|IsInputKeyDown "LeftShift")))
                (Game|SpawnActorfromClass "/Game/Art/ParticleEffects/ClickEffect/BP_ClickEffect.BP_ClickEffect_C" (Math|Conversions|ToTransform(Vector) _location) "AlwaysSpawn" 0 (Variables|Default|GetLocation_Click_Color) (Variables|Default|GetLocation_Click_Speed) 0)
                (else
                  (Audio|PlaySound2D (Variables|Default|GetLocation_Click_InvalidSound)))))))
        (:CastFailed
          (goto _label))))))

(event Input|ActionEvents|InputActionToggleUI
  (params (Key :type Key%20Structure))
  ;[1 1 1] Toggle UI
  (:Pressed
    (bind _returnvalue (Class|RTSPlayerController|GetRTSHUDBase))
    (Class|RTSHUDBase|ToggleVisible _returnvalue)))

(event Input|ActionEvents|InputActionStop
  (params (Key :type Key%20Structure))
  ;[1 1 1] Stop command
  (:Pressed
    (bind _asrts_game_state_bp (Utilities|Casting|CastToRTS_GameState_BP (Game|GetGameState)))
    (for _array_element (Variables|/Script/Wipgate.RTS_GameState|GetSelectedEntities _asrts_game_state_bp)
      (bind _asai_unit_controller (Utilities|Casting|CastToAI_UnitController (AI|GetAIController _array_element)))
      (Class|RTSAIController|AddCommandStop _asai_unit_controller))))

(event Input|ActionEvents|InputActionPrimaryClick
  (params (Key :type Key%20Structure))
  (bind _returnvalue (Game|GetPlayerController 0))
  (bind _hitresult (Game|Player|GetHitResultUnderCursorbyChannel _returnvalue "TraceTypeQuery2" true))
  (bind (_bblockinghit _binitialoverlap _time _distance _location _impactpoint _normal _impactnormal _physmat _hitactor) (Collision|BreakHitResult _hitresult))
  ;[1 1 1] Attack Move
  (:Pressed
    (if (Game|Player|IsInputKeyDown "Q")
      (Utilities|Casting|CastToRTS_Entity _hitactor
        (:CastFailed
          (bind _newparam (CallFunction|GetSquadFormation _location))
          (Variables|Default|SetSquadFormation _newparam)
          (bind _asrts_game_state_bp (Utilities|Casting|CastToRTS_GameState_BP (Game|GetGameState)))
          (for _array_element (Variables|/Script/Wipgate.RTS_GameState|GetSelectedEntities _asrts_game_state_bp)
            (bind _asai_unit_controller (Utilities|Casting|CastToAI_UnitController (AI|GetAIController _array_element)))
            (Class|RTSAIController|AddCommandAttackMove _asai_unit_controller (.Value (Utilities|Map|Find (Variables|Default|GetSquadFormation) _array_element)) false false)
            (Game|SpawnActorfromClass "/Game/Art/ParticleEffects/ClickEffect/BP_ClickEffect.BP_ClickEffect_C" (Math|Conversions|ToTransform(Vector) _location) "AlwaysSpawn" 0 (Variables|Default|GetAttackMove_Color) (Variables|Default|GetLocation_Click_Speed) 0)))))))

(event Input|ActionEvents|InputActionPauseGame
  (params (Key :type Key%20Structure))
  ;[1 1 1] Pause game
  (:Pressed
    (bind _returnvalue (Class|RTSPlayerController|GetRTSHUDBase))
    (bind _asrts_hud_bp (Utilities|Casting|CastToRTS_HUD_BP _returnvalue))
    (Default|TogglePauseMenu _asrts_hud_bp)))

(fn ConstructionScript)

(fn SetFlockManagerReference
  (params (FlockManager :type Object%20Object%20Reference%20%28by%20ref%29))
  (Variables|Default|SetFLOCK_MANAGER_REF FlockManager))

(fn AbilityNotonCooldown
  (params (Ability :type Ability%20Object%20Reference))
  (return (>= (Variables|/Script/Wipgate.Ability|GetCooldownElapsed Ability) (Variables|/Script/Wipgate.Ability|GetCooldown Ability))))

(fn OnAbilitySelected
  (params (Ability :type Ability%20Object%20Reference))
  (if (Utilities|IsValid Ability)
    (if (Utilities|IsValid (Variables|Default|GetSelectedAbility))
      (Class|Ability|Deselect (Variables|Default|GetSelectedAbility))
      (if (!= (Variables|Default|GetSelectedAbility) Ability)
        (if (CallFunction|AbilityNotonCooldown Ability)
          _
          (else
            (Variables|Default|SetSelectedAbility 0 :!label _label)
            (return false false)))
        (else
          (goto _label)))
      (elif (CallFunction|AbilityNotonCooldown Ability)
        _
        (else
          (return false false))))
    (if (Utilities|Enum|Equal(Enum) (Variables|/Script/Wipgate.Ability|GetType Ability) "E_SELF")
      (Class|Ability|Activate Ability)
      (return false true)
      (else
        (bind _output_get (Variables|Default|SetSelectedAbility Ability))
        (Class|Ability|Select _output_get)
        (return true false)))
    (else
      (Development|PrintString "Invalid ability passed to OnAbilitySelected!"))))

(fn GetSpecialistSelected
  (bind _asrts_game_state_bp (Utilities|Casting|CastToRTS_GameState_BP (Game|GetGameState))
    (:then
      (if (== (Utilities|Array|Length (Variables|/Script/Wipgate.RTS_GameState|GetSelectedEntities _asrts_game_state_bp)) 1)
        (return (.AsRTS%20Specialist (Utilities|Casting|CastToRTS_Specialist (Utilities|Array|Get(acopy) (Variables|/Script/Wipgate.RTS_GameState|GetSelectedEntities _asrts_game_state_bp)))) (.bSuccess (Utilities|Casting|CastToRTS_Specialist (Utilities|Array|Get(acopy) (Variables|/Script/Wipgate.RTS_GameState|GetSelectedEntities _asrts_game_state_bp)))))
        (else
          _)))
    (:CastFailed
      _))
  (return 0 false))

(fn PlayAbilityIconAnim
  (params (Ability%20Icon :type RTS%20Ability%20Icon%20Widget%20Object%20Reference) (Selected :type Boolean) (Activated :type Boolean))
  (Utilities|FlowControl|Sequence
    (:then_0
      ;[1 1 1] Deselect any selected ability icon
      (if (Utilities|IsValid (Variables|Default|GetSelected%20Icon))
        (Default|OnDeselected (Variables|Default|GetSelected%20Icon))))
    (:then_1
      (if Activated
        (Default|OnActivated Ability%20Icon)
        (Variables|Default|SetSelected%20Icon 0)
        (elif Selected
          (Default|OnSelected Ability%20Icon)
          (Variables|Default|SetSelected%20Icon Ability%20Icon)
          (else
            (Variables|Default|SetSelected%20Icon 0)))))))

(fn GetSquadFormation
  (params (Target :type Vector))
  (LocalVariables|SetCenter Target)
  (bind _asrts_game_state (Utilities|Casting|CastToRTS_GameState (Game|GetGameState)))
  (LocalVariables|SetWidth (Math|Float|Ceil (Math|Float|Sqrt (Math|Conversions|ToFloat(Integer) (Utilities|Array|Length (Variables|/Script/Wipgate.RTS_GameState|GetSelectedEntities _asrts_game_state))))))
  (LocalVariables|SetHeight (Math|Float|Ceil (Math|Float|Sqrt (Math|Conversions|ToFloat(Integer) (Utilities|Array|Length (Variables|/Script/Wipgate.RTS_GameState|GetSelectedEntities _asrts_game_state))))))
  (LocalVariables|SetTopRight (- (LocalVariables|GetCenter) (Math|Vector|MakeVector (* (LocalVariables|GetOffset) (/ (Math|Conversions|ToFloat(Integer) (LocalVariables|GetWidth)) 2.0)) (* (LocalVariables|GetOffset) (/ (Math|Conversions|ToFloat(Integer) (LocalVariables|GetHeight)) 2.0)) 0.0)))
  (for (_array_element _array_index) (Variables|/Script/Wipgate.RTS_GameState|GetSelectedEntities _asrts_game_state)
    (LocalVariables|SetX (Math|Integer|%(Integer) _array_index (LocalVariables|GetWidth)))
    (LocalVariables|SetY (/ _array_index (LocalVariables|GetHeight)))
    (Utilities|Map|Add (LocalVariables|GetFormation) _array_element (+ (Math|Vector|MakeVector (Math|Conversions|ToFloat(Integer) (* (LocalVariables|GetX) (LocalVariables|GetOffset))) (Math|Conversions|ToFloat(Integer) (* (LocalVariables|GetY) (LocalVariables|GetOffset))) 0.0) (LocalVariables|GetTopRight))))
  (return (LocalVariables|GetFormation)))