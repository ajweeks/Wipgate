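; WipgateGameMode_BP is the RTS game mode, handling level setup and sanity checks at BeginPlay.
; It copies the friendly added troops setting from the RTS_LevelBounds_BP before calling parent BeginPlay, then pushes a sound mix.
; It prints a warning if the map has zero or multiple RTS_MiniMap_BP actors.
; A failed level bounds cast skips all of this, including the parent call.
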(event EventBeginPlay
  (bind _returnvalue (Class|WipgateGameModeBase|GetLevelBounds))
  (bind _asrts_level_bounds_bp (Utilities|Casting|CastToRTS_LevelBounds_BP _returnvalue))
  (Variables|Default|SetUseFriendlyAddedTroops (Variables|/Game/Code/Gameplay/RTS_LevelBounds_BP.RTS_LevelBounds_BP_C|GetUseFriendlyAddedTroops _asrts_level_bounds_bp))
  (|CallParentFunction)
  (Audio|PushSoundMixModifier "/Game/Art/Sounds/SoundMix.SoundMix")
  (bind _outactors (Actor|GetAllActorsOfClass "/Game/Code/User_Interface/RTS_MiniMap_Capture/RTS_MiniMap_BP.RTS_MiniMap_BP_C"))
  (if (<= (Utilities|Array|Length _outactors) 0)
    (Development|PrintString "No RTS_Minimap_BP present in the current map!")
    (elif (> (Utilities|Array|Length _outactors) 1)
      (Development|PrintString "There are more than 1 RTS_Minimap_BPs present in the current map!"))))

(fn ConstructionScript)