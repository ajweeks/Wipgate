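; Base RTS ability actor that handles target selection, cooldown and effect application for a caster.
; Select and Deselect drive ability state, the cursor and a ground-targeting decal, while Tick updates range feedback by target type and counts down cooldown after Activate.
; Helper functions apply tagged unit effects to a target or alignment-filtered units in a radius, replacing non-stackable ones, or spawn AreaOfEffect actors for area effects.
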(event EventBeginPlay
  ;[1 1 1] Create decal
  (CallFunction|InitializeDecal 3e+02))

(event EventDeselect
  (bind _returnvalue (Game|GetPlayerController 0))
  (bind _asrts_player_controller (Utilities|Casting|CastToRTS_PlayerController _returnvalue))
  (bind _cursorref (Variables|/Script/Wipgate.RTS_PlayerController|GetCursorRef _asrts_player_controller))
  ;[1 1 1] Cursor and decal handling on deselection
  (Class|RTSCursor|SetCursorTexture _cursorref (Variables|/Script/Wipgate.RTS_Cursor|GetDefaultTexture _cursorref))
  (Class|WidgetBlueprintLibrary|SetFocustoGameViewport)
  (if (Utilities|Enum|Equal(Enum) (Variables|Default|GetType) "E_TARGET_GROUND")
    (CallFunction|SetDecalEnabled false))
  (if (Utilities|Enum|NotEqual(Enum) (Variables|Default|GetState) "E_ON_COOLDOWN")
    (Variables|Default|SetState "E_AVAILABLE")))

(event EventTick
  (params (DeltaSeconds :type Float%20%28single-precision%29))
  (bind _cooldown (Variables|Default|GetCooldown))
  (bind _defaultsceneroot (Variables|Default|GetDefaultSceneRoot))
  ;[1 1 1] Move decal
  (switch Utilities|FlowControl|Switch|SwitchonEAbilityState (Variables|Default|GetState)
    (:E_SELECTED
      ;;[1 1 1] Reposition based on ability type
      (if true
        (switch Utilities|FlowControl|Switch|SwitchonEAbilityType (Variables|Default|GetType)
          (:E_TARGET_UNIT
            (CallFunction|UpdateCursoronRange :!label _label))
          (:E_TARGET_ENEMY
            (goto _label))
          (:E_TARGET_ALLY
            (goto _label))
          (:E_TARGET_GROUND
            (bind _mouse_pos_world_space (CallFunction|GetMousePosGround))
            (Transformation|SetWorldLocation _defaultsceneroot _mouse_pos_world_space false false)
            (CallFunction|UpdateDecalColor))
          (:E_SELF
            (Transformation|SetWorldLocation _defaultsceneroot (Transformation|GetActorLocation (Variables|Default|Getm_Caster)) false false)))))
    (:E_ON_COOLDOWN
      ;;[1 1 1] Manage active cooldown
      (bind _output_get (Variables|Default|SetCooldownElapsed (+ DeltaSeconds (Variables|Default|GetCooldownElapsed))))
      (if (> _output_get _cooldown)
        (Variables|Default|SetState "E_AVAILABLE")
        (if (> _cooldown 0.0) ; If cooldown > 0, play off cooldown anim
          (bind _asrts_ability_icon_widget (Utilities|Casting|CastToRTS_AbilityIconWidget (Variables|Default|GetIcon)))
          (Default|OnOffCooldown _asrts_ability_icon_widget))))))

(event EventSelect
  ;[1 1 1] Cursor and decal handling on selection
  (if (Utilities|Enum|Equal(Enum) (Variables|Default|GetState) "E_AVAILABLE")
    (Variables|Default|SetState "E_SELECTED")
    (if (Utilities|Enum|Equal(Enum) (Variables|Default|GetType) "E_TARGET_GROUND")
      (Class|RTSCursor|SetCursorTexture (Variables|/Script/Wipgate.RTS_PlayerController|GetCursorRef (.AsRTS%20Player%20Controller (Utilities|Casting|CastToRTS_PlayerController (Game|GetPlayerController 0)))))
      (Class|WidgetBlueprintLibrary|SetFocustoGameViewport)
      (CallFunction|SetDecalEnabled true)
      (else
        (CallFunction|UpdateCursoronRange)))
    (elif (Utilities|Enum|Equal(Enum) (Variables|Default|GetState) "E_ON_COOLDOWN")
      _)))

(event EventActivate
  ;[1 1 1] Ability activate
  (Variables|Default|SetState "E_ON_COOLDOWN")
  (Variables|Default|SetCooldownElapsed 0.0)
  (Variables|Default|SetCooldownPassiveElapsed 0.0)
  (if (Utilities|Enum|Equal(Enum) (Variables|Default|GetType) "E_TARGET_GROUND")
    (CallFunction|SetDecalEnabled false)))

(fn ConstructionScript
  (Variables|Default|SetCooldownElapsed (Variables|Default|GetCooldown))
  (Variables|Default|SetCooldownPassiveElapsed (Variables|Default|GetCooldownPassive)))

(fn SetDecalEnabled
  (params (enabled :type Boolean))
  (Rendering|SetVisibility (Variables|Default|GetTargetAreaDecal) enabled false))

(fn ApplyEffecttoUnitsinArea
  (params (Radius :type Float%20%28single-precision%29) (AffectedStat :type EUnitEffectStat%20Enum :default "HEALING") (EffectType :type EUnitEffectType%20Enum :default "OVER_TIME") (Delay :type Float%20%28single-precision%29) (Magnitude :type Integer) (duration :type Integer) (Relative%20Alignment :type ERelativeAlignment%20Enum :default "E_FRIENDLY") (TickParticle :type Particle%20System%20Object%20Reference) (Start%20Particle :type Particle%20System%20Object%20Reference) (End%20Particle :type Particle%20System%20Object%20Reference) (Constant%20Particle :type Particle%20System%20Object%20Reference) (Tag :type Name) (Effect%20can%20stack :type Boolean))
  (bind _unit (CallFunction|GetUnitsinRange (Transformation|GetWorldLocation (Variables|Default|GetDefaultSceneRoot)) Radius))
  (for _array_element _unit
    (bind _have_relative_alignment (CallFunction|HaveRelativeAlignment _array_element (.AsRTS%20Entity (Utilities|Casting|CastToRTS_Entity (Variables|Default|Getm_Caster))) Relative%20Alignment))
    (if _have_relative_alignment
      (CallFunction|ManageStacking _array_element Effect%20can%20stack Tag)
      (bind _returnvalue (Class|Ability|CreateUnitEffect AffectedStat EffectType Delay Magnitude duration))
      (Class|UnitEffect|SetParticles _returnvalue TickParticle Start%20Particle End%20Particle Constant%20Particle "None")
      (Variables|/Script/Wipgate.UnitEffect|SetTag _returnvalue Tag)
      (Class|RTSEntity|AddUnitEffect _array_element _returnvalue))))

(fn InitializeDecal
  (params (Radius :type Float%20%28single-precision%29))
  (bind _returnvalue (Class|GameplayStatics|SpawnDecalAttached "/Game/Code/Ablities/M_CircleDecal.M_CircleDecal" (Math|Conversions|ToVector(Float) Radius) (Variables|Default|GetDefaultSceneRoot) "None" "0, 0,100.000000" "90.000000, 0, 0" "KeepRelativeOffset" 0.0))
  (Variables|Default|SetTargetAreaDecal _returnvalue)
  (CallFunction|SetDecalEnabled false)
  (Rendering|SetVisibility (Variables|Default|GetDefaultSceneRoot) false true))

(fn ApplyEffecttoTarget
  (params (Target :type RTS%20Unit%20Object%20Reference) (Affected%20stat :type EUnitEffectStat%20Enum :default "HEALING") (Type :type EUnitEffectType%20Enum :default "OVER_TIME") (Delay :type Float%20%28single-precision%29) (Magnitude :type Integer) (Duration :type Integer) (Tick%20Particle :type Particle%20System%20Object%20Reference) (Start%20Particle :type Particle%20System%20Object%20Reference) (End%20Particle :type Particle%20System%20Object%20Reference) (Constant%20Particle :type Particle%20System%20Object%20Reference) (Can%20Effect%20Stack :type Boolean) (Tag :type Name))
  (CallFunction|ManageStacking Target Can%20Effect%20Stack Tag)
  (bind _returnvalue (Class|Ability|CreateUnitEffect Affected%20stat Type Delay Magnitude Duration))
  (Class|UnitEffect|SetParticles _returnvalue Tick%20Particle Start%20Particle End%20Particle Constant%20Particle "None")
  (Variables|/Script/Wipgate.UnitEffect|SetTag _returnvalue Tag)
  (Class|RTSEntity|AddUnitEffect Target _returnvalue))

(fn ApplyEffecttoArea
  (params (Radius :type Float%20%28single-precision%29) (Affected%20Stat :type EUnitEffectStat%20Enum :default "HEALING") (Type :type EUnitEffectType%20Enum :default "OVER_TIME") (Delay :type Float%20%28single-precision%29) (Magnitude :type Integer) (Duration :type Integer) (Relative%20Alignment :type ERelativeAlignment%20Enum :default "E_FRIENDLY") (Tick%20Particle :type Particle%20System%20Object%20Reference) (Start%20Particle :type Particle%20System%20Object%20Reference) (End%20Particle :type Particle%20System%20Object%20Reference) (Constant%20Particle :type Particle%20System%20Object%20Reference))
  (bind _returnvalue (Game|SpawnActorfromClass "/Game/Code/Ablities/AreaOfEffect.AreaOfEffect_C" (Math|Conversions|ToTransform(Vector) (Transformation|GetWorldLocation (Variables|Default|GetDefaultSceneRoot))) "Undefined" 0 Radius Affected%20Stat Type Delay Magnitude Duration Relative%20Alignment (.AsRTS%20Entity (Utilities|Casting|CastToRTS_Entity (Variables|Default|Getm_Caster))) 0))
  (Default|SetEffectParticles _returnvalue Tick%20Particle Start%20Particle End%20Particle Constant%20Particle "None")
  (return _returnvalue))

(fn ApplyEffecttoAreaAroundTarget
  (params (Target :type Actor%20Object%20Reference) (Radius :type Float%20%28single-precision%29) (Affected%20Stat :type EUnitEffectStat%20Enum :default "HEALING") (Type :type EUnitEffectType%20Enum :default "OVER_TIME") (Delay :type Float%20%28single-precision%29) (Magnitude :type Integer) (Duration :type Integer) (Relative%20Alignment :type ERelativeAlignment%20Enum :default "E_FRIENDLY") (Tick%20Particle :type Particle%20System%20Object%20Reference) (Start%20Particle :type Particle%20System%20Object%20Reference) (End%20Particle :type Particle%20System%20Object%20Reference) (Constant%20Particle :type Particle%20System%20Object%20Reference) (Socket%20Name :type Name))
  (bind _returnvalue (Game|SpawnActorfromClass "/Game/Code/Ablities/AreaOfEffect.AreaOfEffect_C" (Transformation|GetWorldTransform (Variables|Default|GetDefaultSceneRoot)) "Undefined" Target Radius Affected%20Stat Type Delay Magnitude Duration Relative%20Alignment (.AsRTS%20Entity (Utilities|Casting|CastToRTS_Entity (Variables|Default|Getm_Caster))) 0))
  (Default|SetEffectParticles _returnvalue Tick%20Particle Start%20Particle End%20Particle Constant%20Particle Socket%20Name)
  (return _returnvalue))

(fn UpdateDecalColor
  (bind _returnvalue (CallFunction|GetDistancetoTarget))
  (if (> _returnvalue (Variables|Default|GetCastRange))
    (bind _returnvalue_2 (Rendering|Material|CreateDynamicMaterialInstance "/Game/Code/Ablities/M_CircleDecal.M_CircleDecal" :!class /Script/Engine.KismetMaterialLibrary))
    (Rendering|Material|SetVectorParameterValue _returnvalue_2 (Utilities|String|StringToName "Color") (Math|Conversions|ToLinearColor(Color) (LocalVariables|GetColorOutOfRange)) :!class /Script/Engine.MaterialInstanceDynamic)
    (Rendering|Components|Decal|SetDecalMaterial (Variables|Default|GetTargetAreaDecal) _returnvalue_2)
    (else
      (bind _returnvalue_3 (Rendering|Material|CreateDynamicMaterialInstance "/Game/Code/Ablities/M_CircleDecal.M_CircleDecal" :!class /Script/Engine.KismetMaterialLibrary))
      (Rendering|Material|SetVectorParameterValue _returnvalue_3 (Utilities|String|StringToName "Color") (Math|Conversions|ToLinearColor(Color) (LocalVariables|GetColorInRange)) :!class /Script/Engine.MaterialInstanceDynamic)
      (Rendering|Components|Decal|SetDecalMaterial (Variables|Default|GetTargetAreaDecal) _returnvalue_3))))

(fn GetDistancetoTarget
  (switch Utilities|FlowControl|Switch|SwitchonEAbilityType "E_TARGET_UNIT"
    (:E_TARGET_UNIT
      _)
    (:E_TARGET_ENEMY
      _)
    (:E_TARGET_ALLY
      _)
    (:E_TARGET_GROUND
      (return (Math|Vector|VectorLength (- (Transformation|GetWorldLocation (Variables|Default|GetDefaultSceneRoot)) (Transformation|GetActorLocation (Variables|Default|Getm_Caster)))))))
  (bind _mouse_pos_world_space (CallFunction|GetMousePosGround))
  (return (Math|Vector|VectorLength (- _mouse_pos_world_space (Transformation|GetActorLocation (Variables|Default|Getm_Caster))))))

(fn UpdateCursoronRange
  (bind _returnvalue (Game|GetPlayerController 0))
  (bind _asrts_player_controller (Utilities|Casting|CastToRTS_PlayerController _returnvalue))
  (bind _cursorref (Variables|/Script/Wipgate.RTS_PlayerController|GetCursorRef _asrts_player_controller))
  (bind _returnvalue_2 (CallFunction|GetDistancetoTarget))
  (if (> _returnvalue_2 (Variables|Default|GetCastRange))
    (Class|RTSCursor|SetCursorTexture _cursorref (Variables|/Script/Wipgate.RTS_Cursor|GetInvalidTexture _cursorref))
    (else
      (Class|RTSCursor|SetCursorTexture _cursorref (Variables|/Script/Wipgate.RTS_Cursor|GetDefaultTexture _cursorref))))
  (Class|WidgetBlueprintLibrary|SetFocustoGameViewport))

(fn SetTargetAlignment
  (params (Relative%20Alignment :type ERelativeAlignment%20Enum :default "E_FRIENDLY"))
  (bind _asrts_entity (Utilities|Casting|CastToRTS_Entity (Variables|Default|Getm_Caster)))
  (switch Utilities|FlowControl|Switch|SwitchonERelativeAlignment Relative%20Alignment
    (:E_FRIENDLY
      (switch Utilities|FlowControl|Switch|SwitchonETeamAlignment (Variables|/Script/Wipgate.RTS_Entity|GetAlignment _asrts_entity)
        (:E_PLAYER
          (return "E_PLAYER"))
        (:E_AGGRESSIVE_AI
          (return "E_AGGRESSIVE_AI"))))
    (:E_ENEMY
      (switch Utilities|FlowControl|Switch|SwitchonETeamAlignment (Variables|/Script/Wipgate.RTS_Entity|GetAlignment _asrts_entity)
        (:E_PLAYER
          (return "E_AGGRESSIVE_AI"))
        (:E_AGGRESSIVE_AI
          (return "E_PLAYER"))))))

(fn GetTargetHalfHeight
  (params (Object :type Object%20Object%20Reference))
  (bind _asrts_unit (Utilities|Casting|CastToRTS_Unit Object)
    (:then
      _)
    (:CastFailed
      _))
  (return (Math|Vector|MakeVector 0.0 0.0 (Components|Capsule|GetScaledCapsuleHalfHeight (Actor|GetComponentbyClass _asrts_unit "/Script/Engine.CapsuleComponent")))))

(fn ManageStacking
  (params (Target%20Unit :type RTS%20Unit%20Object%20Reference) (Can%20Stack :type Boolean) (Tag :type Name))
  (Utilities|IsValid Target%20Unit
    (:Is%20Valid
      (if (Utilities|Name|Equal(Name) Tag "None")
        _
        (elif (not Can%20Stack)
          (bind _returnvalue (Class|RTSEntity|HasEffectwithTag Target%20Unit Tag))
          (if _returnvalue
            (Class|RTSEntity|RemoveUnitEffectwithTag Target%20Unit Tag)))))
    (:Is%20Not%20Valid
      _))
  (return))