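; Blueprint function library of shared helpers for an RTS game, covering cursor picking, entity queries and UI styling.
; Sphere overlaps on Pawns gather units in range or entities filtered by team alignment, and a distance loop picks the closest entity.
; The opposing-alignment helper returns inside its enum loop, at the first differing non-neutral alignment.
; Other helpers return the slightly raised ground point under the cursor and rebuild button styles with new size, draw type and margin.
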(fn GetMousePosGround
  (return (+ (.Location (Collision|BreakHitResult (.HitResult (Class|PlayerController|GetHitResultUnderCursorforObjects (Game|GetPlayerController 0) (Utilities|Array|MakeArray "ObjectTypeQuery1") true)))) "0, 0,10.000000")))

(fn DetectUnitswithAlignment
  (params (WorldContextObject :type Actor%20Object%20Reference%20%28by%20ref%29) (Position :type Vector) (Range :type Float%20%28single-precision%29) (ActorsToIgnore :type Array%20of%20Actor%20Object%20References) (Alignment :type Array%20of%20EAlignment%20Enums :default "E_FRIENDLY"))
  (bind (_outactors _returnvalue) (Collision|SphereOverlapActors WorldContextObject Position Range (Utilities|Array|MakeArray "ObjectTypeQuery3") "/Script/Wipgate.RTS_Entity" ActorsToIgnore))
  (if _returnvalue
    (for _array_element _outactors
      (bind _asrts_entity (Utilities|Casting|CastToRTS_Entity _array_element))
      (if (!= (Utilities|Array|FindItem Alignment (.alignment (Variables|/Script/Wipgate.RTS_Entity|GetTeam _asrts_entity))) -1)
        (Utilities|Array|Add (LocalVariables|GetActorsWithAlignment) _asrts_entity)))
    (return (> (Utilities|Array|Length (LocalVariables|GetActorsWithAlignment)) 0) (LocalVariables|GetActorsWithAlignment))
    (else
      (return false 0))))

(fn GetNonCharacterAlignments
  (params (Alingment :type EAlignment%20Enum :default "E_FRIENDLY") (IncludeNeutrals :type Boolean))
  (bind _enumvalue (|ForEachEAlignment)
    (:LoopBody
      (if (Utilities|Enum|NotEqual(Enum) Alingment _enumvalue)
        (if (Utilities|Enum|NotEqual(Enum) _enumvalue "E_NEUTRAL")
          (Utilities|Array|Add (LocalVariables|GetAlignment) _enumvalue)
          (return (LocalVariables|GetAlignment))
          (elif IncludeNeutrals
            (Utilities|Array|Add (LocalVariables|GetAlignment) "E_NEUTRAL")))))))

(fn GetUnitsinRange
  (params (Location :type Vector) (Radius :type Float%20%28single-precision%29))
  (bind _unitcharacters (LocalVariables|GetUnitCharacters))
  (bind (_outactors _returnvalue) (Collision|SphereOverlapActors 0 Location Radius (Utilities|Array|MakeArray "ObjectTypeQuery3") "/Script/Wipgate.RTS_Unit"))
  (if _returnvalue
    (for _array_element _outactors
      (bind _asrts_unit (Utilities|Casting|CastToRTS_Unit _array_element))
      (Utilities|Array|Add _unitcharacters _asrts_unit))
    (return _unitcharacters)))

(fn GetClosestEntity
  (params (Entity :type RTS%20Entity%20Object%20Reference) (Others :type Array%20of%20RTS%20Entity%20Object%20References))
  (for _array_element Others
    (if (< (Transformation|GetDistanceTo Entity _array_element) (LocalVariables|GetshortestDistance))
      (LocalVariables|SetshortestDistance (Transformation|GetDistanceTo Entity _array_element))
      (LocalVariables|SetclosestEntity _array_element)))
  (return (LocalVariables|GetclosestEntity)))

(fn SetButtonStyle
  (params (Button :type Button%20Object%20Reference) (Imge%20Size :type Vector%202D%20Structure) (Draw%20Type :type ESlateBrushDrawType%20Enum :default "NoDrawType") (Margin :type Margin%20Structure))
  (bind _widgetstyle (Variables|/Script/UMG.Button|GetWidgetStyle Button))
  (return (Utilities|Struct|MakeButtonStyle (Utilities|Struct|MakeSlateBrush Imge%20Size Margin (.tintcolor (.normal _widgetstyle)) (.resourceobject (.normal _widgetstyle)) Draw%20Type (.tiling (.normal _widgetstyle)) (.mirroring (.normal _widgetstyle))) (Utilities|Struct|MakeSlateBrush Imge%20Size Margin (.tintcolor (.hovered _widgetstyle)) (.resourceobject (.hovered _widgetstyle)) Draw%20Type (.tiling (.hovered _widgetstyle)) (.mirroring (.hovered _widgetstyle))) (Utilities|Struct|MakeSlateBrush Imge%20Size Margin (.tintcolor (.pressed _widgetstyle)) (.resourceobject (.pressed _widgetstyle)) Draw%20Type (.tiling (.pressed _widgetstyle)) (.mirroring (.pressed _widgetstyle))) (Utilities|Struct|MakeSlateBrush Imge%20Size Margin (.tintcolor (.disabled _widgetstyle)) (.resourceobject (.disabled _widgetstyle)) Draw%20Type (.tiling (.disabled _widgetstyle)) (.mirroring (.disabled _widgetstyle))) (.normalpadding _widgetstyle) (.pressedpadding _widgetstyle) (.pressedslatesound _widgetstyle) (.hoveredslatesound _widgetstyle))))