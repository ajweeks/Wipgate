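; RTS camera pawn that views the game through a spring arm with adjustable length.
; The construction script sets the arm to a configurable starting length.
; A Zoom function shortens or lengthens the arm by a delta, clamped between minimum and maximum lengths.
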(fn ConstructionScript
  (Variables|/Script/Engine.SpringArmComponent|SetTargetArmLength (Variables|Default|GetSpringArm) (Variables|Default|GetStartingArmLength)))

(fn Zoom
  (params (DeltaZoom :type Float%20%28single-precision%29))
  (Variables|/Script/Engine.SpringArmComponent|SetTargetArmLength (Variables|Default|GetSpringArm) (Math|Float|Clamp(Float) (- (Variables|/Script/Engine.SpringArmComponent|GetTargetArmLength (Variables|Default|GetSpringArm)) DeltaZoom) (Variables|Default|GetMinArmLength) (Variables|Default|GetMaxArmLength))))