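; RTS player controller that turns input into stop, attack and move commands for the AI controllers of units selected in the game state.
; Right-click traces under the cursor to force attacks on entities or issue Shift-queueable moves on navigable ground, with click effect or invalid sound.
; Ability button events use the first selected specialist, checking cooldown, then activating self-cast abilities or selecting others.
; It also toggles the HUD and stores a flock manager reference.
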(event EventOnAbilityPassiveButtonPress
  (if (not (Utilities|IsValid (Variables|Default|Getm_SelectedAbility)))
    (bind _asrts_game_state_bp (Utilities|Casting|CastToRTS_GameState_BP (Game|GetGameState)))
    (bind _asrts_specialist (Utilities|Casting|CastToRTS_Specialist (Utilities|Array|Get(acopy) (Variables|/Script/Wipgate.RTS_GameState|GetSelectedEntities _asrts_game_state_bp))))
    (if (>= (Variables|/Script/Wipgate.Ability|GetCooldownElapsed (Variables|/Script/Wipgate.RTS_Specialist|GetAbilityPassive _asrts_specialist)) (Variables|/Script/Wipgate.Ability|GetCooldown (Variables|/Script/Wipgate.RTS_Specialist|GetAbilityPassive _asrts_specialist)))
      (if (Utilities|Enum|Equal(Enum) (Variables|/Script/Wipgate.Ability|GetType (Variables|/Script/Wipgate.RTS_Specialist|GetAbilityPassive _asrts_specialist)) "E_SELF")
        (Class|Ability|Activate (Variables|/Script/Wipgate.RTS_Specialist|GetAbilityPassive _asrts_specialist))
        (else
          (bind _output_get (Variables|Default|Setm_SelectedAbility (Variables|/Script/Wipgate.RTS_Specialist|GetAbilityPassive _asrts_specialist)))
          (Class|Ability|Select _output_get))))))

(event EventOnAbilityConstructButtonPress
  (if (not (Utilities|IsValid (Variables|Default|Getm_SelectedAbility)))
    (bind _asrts_game_state_bp (Utilities|Casting|CastToRTS_GameState_BP (Game|GetGameState)))
    (bind _asrts_specialist (Utilities|Casting|CastToRTS_Specialist (Utilities|Array|Get(acopy) (Variables|/Script/Wipgate.RTS_GameState|GetSelectedEntities _asrts_game_state_bp))))
    (Development|PrintString (Utilities|String|ToString(Float) (Variables|/Script/Wipgate.Ability|GetCooldownElapsed (Variables|/Script/Wipgate.RTS_Specialist|GetAbilityConstruct _asrts_specialist))))
    (if (>= (Variables|/Script/Wipgate.Ability|GetCooldownElapsed (Variables|/Script/Wipgate.RTS_Specialist|GetAbilityConstruct _asrts_specialist)) (Variables|/Script/Wipgate.Ability|GetCooldown (Variables|/Script/Wipgate.RTS_Specialist|GetAbilityConstruct _asrts_specialist)))
      (if (Utilities|Enum|Equal(Enum) (Variables|/Script/Wipgate.Ability|GetType (Variables|/Script/Wipgate.RTS_Specialist|GetAbilityConstruct _asrts_specialist)) "E_SELF")
        (Class|Ability|Activate (Variables|/Script/Wipgate.RTS_Specialist|GetAbilityConstruct _asrts_specialist))
        (else
          (bind _output_get (Variables|Default|Setm_SelectedAbility (Variables|/Script/Wipgate.RTS_Specialist|GetAbilityConstruct _asrts_specialist)))
          (Class|Ability|Select _output_get))))))

(event EventOnAbilityActiveButtonPress
  (bind _asrts_game_state_bp (Utilities|Casting|CastToRTS_GameState_BP (Game|GetGameState)))
  (bind _asrts_specialist (Utilities|Casting|CastToRTS_Specialist (Utilities|Array|Get(acopy) (Variables|/Script/Wipgate.RTS_GameState|GetSelectedEntities _asrts_game_state_bp))))
  (if (Utilities|IsValid (Variables|Default|Getm_SelectedAbility))
    (Class|Ability|Deselect (Variables|Default|Getm_SelectedAbility))
    (if (== (Variables|Default|Getm_SelectedAbility) (Variables|/Script/Wipgate.RTS_Specialist|GetAbilityActive _asrts_specialist))
      _)
    (elif (>= (Variables|/Script/Wipgate.Ability|GetCooldownElapsed (Variables|/Script/Wipgate.RTS_Specialist|GetAbilityActive _asrts_specialist)) (Variables|/Script/Wipgate.Ability|GetCooldown (Variables|/Script/Wipgate.RTS_Specialist|GetAbilityActive _asrts_specialist)))
      (if (Utilities|Enum|Equal(Enum) (Variables|/Script/Wipgate.Ability|GetType (Variables|/Script/Wipgate.RTS_Specialist|GetAbilityActive _asrts_specialist)) "E_SELF")
        (Class|Ability|Activate (Variables|/Script/Wipgate.RTS_Specialist|GetAbilityActive _asrts_specialist))
        (else
          (bind _output_get (Variables|Default|Setm_SelectedAbility (Variables|/Script/Wipgate.RTS_Specialist|GetAbilityActive _asrts_specialist)))
          (Class|Ability|Select _output_get))))))

(event Input|ActionEvents|InputActionSecondaryClick
  (params (Key :type Key%20Structure))
  (bind _returnvalue (Game|GetPlayerController 0))
  (bind _hitresult (Game|Player|GetHitResultUnderCursorbyChannel _returnvalue "TraceTypeQuery2" true))
  (bind (_bblockinghit _binitialoverlap _time _distance _location _impactpoint _normal _impactnormal _physmat _hitactor) (Collision|BreakHitResult _hitresult))
  ;[1 1 1] Right-click movement
  ;;[1 1 1] Get Gamestate on right mouse
  (:Pressed
    (bind _asrts_game_state_bp (Utilities|Casting|CastToRTS_GameState_BP (Game|GetGameState)))
    ;;[1 1 1] Check if user has units selected
    (if (> (Utilities|Array|Length (Variables|/Script/Wipgate.RTS_GameState|GetSelectedEntities _asrts_game_state_bp)) 0)
      ;;[1 1 1] Raycast from mouse
      (bind _asrts_entity (Utilities|Casting|CastToRTS_Entity _hitactor)
        (:then
          ;;[1 1 1] If selection was character
          (for _array_element (Variables|/Script/Wipgate.RTS_GameState|GetSelectedEntities _asrts_game_state_bp)
            (if (!= _array_element _asrts_entity)
              (bind _asai_unit_controller (Utilities|Casting|CastToAI_UnitController (AI|GetAIController _array_element)))
              (Default|AddCommand:Attack _asai_unit_controller _asrts_entity false true))))
        (:CastFailed
          (if (.ReturnValue (AI|Navigation|ProjectPointtoNavigation _location 0 0 "0, 0, 0"))
            ;;[1 1 1] If selection was non-character
            (for _array_element_2 (Variables|/Script/Wipgate.RTS_GameState|GetSelectedEntities _asrts_game_state_bp)
              (bind _asai_unit_controller_2 (Utilities|Casting|CastToAI_UnitController (AI|GetAIController _array_element_2)))
              (Default|AddCommand:MovetoLocation _asai_unit_controller_2 (Game|Player|IsInputKeyDown "LeftShift") _location))
            (Game|SpawnActorfromClass "/Game/Art/ParticleEffects/ClickEffect/BP_ClickEffect.BP_ClickEffect_C" (Math|Conversions|ToTransform(Vector) _location) "AlwaysSpawn" 0 (Variables|Default|GetLocation_Click_Color) (Variables|Default|GetLocation_Click_Speed) 0)
            (else
              (Audio|PlaySound2D (Variables|Default|GetLocation_Click_InvalidSound)))))))))

(event Input|ActionEvents|InputActionToggleUI
  (params (Key :type Key%20Structure))
  (:Pressed
    (bind _returnvalue (Class|RTSPlayerController|GetHUD))
    (Class|RTSHUDBase|ToggleVisible _returnvalue)))

(event Input|ActionEvents|InputActionStop
  (params (Key :type Key%20Structure))
  ;[1 1 1] Stop command
  (:Pressed
    (bind _asrts_game_state_bp (Utilities|Casting|CastToRTS_GameState_BP (Game|GetGameState)))
    (for _array_element (Variables|/Script/Wipgate.RTS_GameState|GetSelectedEntities _asrts_game_state_bp)
      (bind _asai_unit_controller (Utilities|Casting|CastToAI_UnitController (AI|GetAIController _array_element)))
      (Default|AddCommand:Stop _asai_unit_controller))))

(fn ConstructionScript)

(fn SetFlockManagerReference
  (params (FlockManager :type Flock%20Manager%20BP%20Object%20Reference%20%28by%20ref%29))
  (Variables|Default|SetFLOCK_MANAGER_REF FlockManager))