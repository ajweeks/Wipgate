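; Base RTS ability actor that handles selection, targeting feedback, cooldown and effect application for a caster.
; Select, Deselect and Activate switch between available, selected and cooldown states, with Tick counting down the cooldown.
; While selected, Tick shows cast range via the cursor or, for ground targeting, a mouse-following decal recolored through new dynamic materials.
; Helper functions apply unit effects to targets or areas, or spawn AreaOfEffect actors, resolving alignment relative to the caster's team.
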(event EventBeginPlay
  ;[1 1 1] Create decal
  (CallFunction|InitializeDecal 3e+02))

(event EventDeselect
  ;[1 1 1] Cursor and decal handling on deselection
  (Variables|/Script/Engine.PlayerController|SetCurrentMouseCursor (Game|GetPlayerController 0) "Default")
  (Class|WidgetBlueprintLibrary|SetFocustoGameViewport)
  (if (Utilities|Enum|Equal(Enum) (Variables|Default|GetType) "E_TARGET_GROUND")
    (CallFunction|SetDecalEnabled false))
  (if (Utilities|Enum|NotEqual(Enum) (Variables|Default|GetState) "E_ON_COOLDOWN")
    (Variables|Default|SetState "E_AVAILABLE")))

(event EventTick
  (params (DeltaSeconds :type Float%20%28single-precision%29))
  (bind _defaultsceneroot (Variables|Default|GetDefaultSceneRoot))
  ;[1 1 1] Move decal
  (switch Utilities|FlowControl|Switch|SwitchonEAbilityState (Variables|Default|GetState)
    (:E_SELECTED
      ;;[1 1 1] Reposition based on ability type
      (if true
        (switch Utilities|FlowControl|Switch|SwitchonEAbilityType (Variables|Default|GetType)
          (:E_TARGET_UNIT
            (CallFunction|UpdateCursoronRange :!label _label))
          (:E_TARGET_ENEMY
            (goto _label))
          (:E_TARGET_ALLY
            (goto _label))
          (:E_TARGET_GROUND
            (bind _newparam (CallFunction|GetMousePosGround))
            (Transformation|SetWorldLocation _defaultsceneroot _newparam false false)
            (CallFunction|UpdateDecalColor))
          (:E_SELF
            (Transformation|SetWorldLocation _defaultsceneroot (Transformation|GetActorLocation (Variables|Default|Getm_Caster)) false false)))))
    (:E_ON_COOLDOWN
      ;;[1 1 1] Manage active cooldown
      (bind _output_get (Variables|Default|SetCooldownElapsed (+ DeltaSeconds (Variables|Default|GetCooldownElapsed))))
      (if (> _output_get (Variables|Default|GetCooldown))
        (Variables|Default|SetState "E_AVAILABLE")))))

(event EventSelect
  ;[1 1 1] Cursor and decal handling on selection
  (if (Utilities|Enum|Equal(Enum) (Variables|Default|GetState) "E_AVAILABLE")
    (Variables|Default|SetState "E_SELECTED")
    (if (Utilities|Enum|Equal(Enum) (Variables|Default|GetType) "E_TARGET_GROUND")
      (Variables|/Script/Engine.PlayerController|SetCurrentMouseCursor (Game|GetPlayerController 0) "None")
      (Class|WidgetBlueprintLibrary|SetFocustoGameViewport)
      (CallFunction|SetDecalEnabled true)
      (else
        (CallFunction|UpdateCursoronRange)))
    (elif (Utilities|Enum|Equal(Enum) (Variables|Default|GetState) "E_ON_COOLDOWN")
      _)))

(event EventActivate
  ;[1 1 1] Ability activate
  (Variables|Default|SetState "E_ON_COOLDOWN")
  (Variables|Default|SetCooldownElapsed 0.0)
  (if (Utilities|Enum|Equal(Enum) (Variables|Default|GetType) "E_TARGET_GROUND")
    (CallFunction|SetDecalEnabled false)))

(fn ConstructionScript
  (Variables|Default|SetCooldownElapsed (Variables|Default|GetCooldown))
  (Variables|Default|SetCooldownPassiveElapsed (Variables|Default|GetCooldownPassive)))

(fn SetDecalEnabled
  (params (enabled :type Boolean))
  (Rendering|SetVisibility (Variables|Default|GetTargetAreaDecal) enabled false))

(fn ApplyEffecttoUnitsinArea
  (params (Radius :type Float%20%28single-precision%29) (AffectedStat :type EUnitEffectStat%20Enum :default "HEALING") (EffectType :type EUnitEffectType%20Enum :default "OVER_TIME") (Delay :type Float%20%28single-precision%29) (Magnitude :type Integer) (duration :type Integer) (Relative%20Alignment :type EAlignment%20Enum :default "E_ENEMY") (TickParticle :type Particle%20System%20Object%20Reference) (Start%20Particle :type Particle%20System%20Object%20Reference) (End%20Particle :type Particle%20System%20Object%20Reference) (Constant%20Particle :type Particle%20System%20Object%20Reference))
  (bind _absolute_target_alignment (CallFunction|SetTargetAlignment Relative%20Alignment))
  (LocalVariables|SettargetAlignment _absolute_target_alignment)
  (bind _unit (CallFunction|GetUnitsinRange (Transformation|GetWorldLocation (Variables|Default|GetDefaultSceneRoot)) Radius))
  (for _array_element _unit
    (if (Utilities|Enum|Equal(Enum) (.alignment (Variables|/Script/Wipgate.RTS_Entity|GetTeam _array_element)) (LocalVariables|GettargetAlignment))
      (bind _returnvalue (Class|Ability|CreateUnitEffect AffectedStat EffectType Delay Magnitude duration))
      (Class|UnitEffect|SetParticles _returnvalue TickParticle Start%20Particle End%20Particle Constant%20Particle "None")
      (Class|RTSEntity|AddUnitEffect _array_element _returnvalue))))

(fn InitializeDecal
  (params (Radius :type Float%20%28single-precision%29))
  (bind _returnvalue (Class|GameplayStatics|SpawnDecalAttached "/Game/Code/Blueprints/Ablities/M_CircleDecal.M_CircleDecal" (Math|Conversions|ToVector(Float) Radius) (Variables|Default|GetDefaultSceneRoot) "None" "0, 0,100.000000" "90.000000, 0, 0" "KeepRelativeOffset" 0.0))
  (Variables|Default|SetTargetAreaDecal _returnvalue)
  (CallFunction|SetDecalEnabled false)
  (Rendering|SetVisibility (Variables|Default|GetDefaultSceneRoot) false true))

(fn ApplyEffecttoTarget
  (params (Target :type RTS%20Unit%20Object%20Reference) (Affected%20stat :type EUnitEffectStat%20Enum :default "HEALING") (Type :type EUnitEffectType%20Enum :default "OVER_TIME") (Delay :type Float%20%28single-precision%29) (Magnitude :type Integer) (Duration :type Integer) (Tick%20Particle :type Particle%20System%20Object%20Reference) (Start%20Particle :type Particle%20System%20Object%20Reference) (End%20Particle :type Particle%20System%20Object%20Reference) (Constant%20Particle :type Particle%20System%20Object%20Reference))
  (bind _returnvalue (Class|Ability|CreateUnitEffect Affected%20stat Type Delay Magnitude Duration))
  (Class|UnitEffect|SetParticles _returnvalue Tick%20Particle Start%20Particle End%20Particle Constant%20Particle "None")
  (Class|RTSEntity|AddUnitEffect Target _returnvalue))

(fn ApplyEffecttoArea
  (params (Radius :type Float%20%28single-precision%29) (Affected%20Stat :type EUnitEffectStat%20Enum :default "HEALING") (Type :type EUnitEffectType%20Enum :default "OVER_TIME") (Delay :type Float%20%28single-precision%29) (Magnitude :type Integer) (Duration :type Integer) (Relative%20Alignment :type EAlignment%20Enum :default "E_FRIENDLY") (Tick%20Particle :type Particle%20System%20Object%20Reference) (Start%20Particle :type Particle%20System%20Object%20Reference) (End%20Particle :type Particle%20System%20Object%20Reference) (Constant%20Particle :type Particle%20System%20Object%20Reference))
  (bind _absolute_target_alignment (CallFunction|SetTargetAlignment Relative%20Alignment))
  (bind _returnvalue (Game|SpawnActorfromClass "/Game/Code/Blueprints/Ablities/AreaOfEffect.AreaOfEffect_C" (Math|Conversions|ToTransform(Vector) (Transformation|GetWorldLocation (Variables|Default|GetDefaultSceneRoot))) "Undefined" 0 Radius Affected%20Stat Type Delay Magnitude Duration _absolute_target_alignment 0))
  (Default|SetEffectParticles _returnvalue Tick%20Particle Start%20Particle End%20Particle Constant%20Particle "None")
  (return _returnvalue))

(fn ApplyEffecttoAreaAroundTarget
  (params (Target :type Actor%20Object%20Reference) (Radius :type Float%20%28single-precision%29) (Affected%20Stat :type EUnitEffectStat%20Enum :default "HEALING") (Type :type EUnitEffectType%20Enum :default "OVER_TIME") (Delay :type Float%20%28single-precision%29) (Magnitude :type Integer) (Duration :type Integer) (Relative%20Alignment :type EAlignment%20Enum :default "E_FRIENDLY") (Tick%20Particle :type Particle%20System%20Object%20Reference) (Start%20Particle :type Particle%20System%20Object%20Reference) (End%20Particle :type Particle%20System%20Object%20Reference) (Constant%20Particle :type Particle%20System%20Object%20Reference) (Socket%20Name :type Name))
  (bind _absolute_target_alignment (CallFunction|SetTargetAlignment Relative%20Alignment))
  (bind _returnvalue (Game|SpawnActorfromClass "/Game/Code/Blueprints/Ablities/AreaOfEffect.AreaOfEffect_C" (Transformation|GetWorldTransform (Variables|Default|GetDefaultSceneRoot)) "Undefined" Target Radius Affected%20Stat Type Delay Magnitude Duration _absolute_target_alignment 0))
  (Default|SetEffectParticles _returnvalue Tick%20Particle Start%20Particle End%20Particle Constant%20Particle Socket%20Name)
  (return _returnvalue))

(fn UpdateDecalColor
  (bind _returnvalue (CallFunction|GetDistancetoTarget))
  (if (> _returnvalue (Variables|Default|GetCastRange))
    (bind _returnvalue_2 (Rendering|Material|CreateDynamicMaterialInstance "/Game/Code/Blueprints/Ablities/M_CircleDecal.M_CircleDecal" :!class /Script/Engine.KismetMaterialLibrary))
    (Rendering|Material|SetVectorParameterValue _returnvalue_2 (Utilities|String|StringToName "Color") (Math|Conversions|ToLinearColor(Color) (LocalVariables|GetColorOutOfRange)) :!class /Script/Engine.MaterialInstanceDynamic)
    (Rendering|Components|Decal|SetDecalMaterial (Variables|Default|GetTargetAreaDecal) _returnvalue_2)
    (else
      (bind _returnvalue_3 (Rendering|Material|CreateDynamicMaterialInstance "/Game/Code/Blueprints/Ablities/M_CircleDecal.M_CircleDecal" :!class /Script/Engine.KismetMaterialLibrary))
      (Rendering|Material|SetVectorParameterValue _returnvalue_3 (Utilities|String|StringToName "Color") (Math|Conversions|ToLinearColor(Color) (LocalVariables|GetColorInRange)) :!class /Script/Engine.MaterialInstanceDynamic)
      (Rendering|Components|Decal|SetDecalMaterial (Variables|Default|GetTargetAreaDecal) _returnvalue_3))))

(fn GetDistancetoTarget
  (switch Utilities|FlowControl|Switch|SwitchonEAbilityType "E_TARGET_UNIT"
    (:E_TARGET_UNIT
      _)
    (:E_TARGET_ENEMY
      _)
    (:E_TARGET_ALLY
      _)
    (:E_TARGET_GROUND
      (return (Math|Vector|VectorLength (- (Transformation|GetWorldLocation (Variables|Default|GetDefaultSceneRoot)) (Transformation|GetActorLocation (Variables|Default|Getm_Caster)))))))
  (bind _newparam (CallFunction|GetMousePosGround))
  (return (Math|Vector|VectorLength (- _newparam (Transformation|GetActorLocation (Variables|Default|Getm_Caster))))))

(fn UpdateCursoronRange
  (bind _returnvalue (CallFunction|GetDistancetoTarget))
  (if (> _returnvalue (Variables|Default|GetCastRange))
    (Variables|/Script/Engine.PlayerController|SetCurrentMouseCursor (Game|GetPlayerController 0) "SlashedCircle")
    (else
      (Variables|/Script/Engine.PlayerController|SetCurrentMouseCursor (Game|GetPlayerController 0) "CardinalCross")))
  (Class|WidgetBlueprintLibrary|SetFocustoGameViewport))

(fn SetTargetAlignment
  (params (Relative%20Target%20Alignment :type EAlignment%20Enum :default "E_FRIENDLY"))
  (bind _asrts_entity (Utilities|Casting|CastToRTS_Entity (Variables|Default|Getm_Caster)))
  (switch Utilities|FlowControl|Switch|SwitchonEAlignment Relative%20Target%20Alignment
    (:E_FRIENDLY
      (switch Utilities|FlowControl|Switch|SwitchonEAlignment (.alignment (Variables|/Script/Wipgate.RTS_Entity|GetTeam _asrts_entity))
        (:E_FRIENDLY
          (return "E_FRIENDLY"))
        (:E_ENEMY
          (return "E_ENEMY"))))
    (:E_ENEMY
      (switch Utilities|FlowControl|Switch|SwitchonEAlignment (.alignment (Variables|/Script/Wipgate.RTS_Entity|GetTeam _asrts_entity))
        (:E_FRIENDLY
          (return "E_ENEMY"))
        (:E_ENEMY
          (return "E_FRIENDLY"))))))

(fn GetTargetHalfHeight
  (params (Object :type Object%20Object%20Reference))
  (bind _asrts_unit (Utilities|Casting|CastToRTS_Unit Object)
    (:then
      _)
    (:CastFailed
      _))
  (return (Math|Vector|MakeVector 0.0 0.0 (Components|Capsule|GetScaledCapsuleHalfHeight (Actor|GetComponentbyClass _asrts_unit "/Script/Engine.CapsuleComponent")))))