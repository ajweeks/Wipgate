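; Area-of-effect actor for RTS abilities that applies a timed unit effect to units of the target alignment inside its radius.
; Follows its owner near the capsule base, with sphere collider and plane sized from Radius.
; Overlap creates a per-unit effect with the remaining delay, mapped by unit and removed on exit, expiry or destruction.
; SetEffectParticles also updates existing effects, since overlaps can fire before initialization.
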(event EventDestroyed
  (CallFunction|DestroyAreaOfEffect))

(event Collision|EventActorEndOverlap
  (params (OtherActor :type Actor%20Object%20Reference))
  ;[1 1 1] Remove Effect on end overlap
  (bind _asrts_unit (Utilities|Casting|CastToRTS_Unit OtherActor))
  (Class|RTSEntity|RemoveUnitEffect _asrts_unit (.Value (Utilities|Map|Find (Variables|Default|GetUnitsAndEffects) _asrts_unit))))

(event Collision|EventActorBeginOverlap
  (params (OtherActor :type Actor%20Object%20Reference))
  (bind _delay (Variables|Default|GetDelay))
  ;[1 1 1] Create effect for each unit and apply
  (bind _asrts_unit (Utilities|Casting|CastToRTS_Unit OtherActor))
  (if (Utilities|Enum|Equal(Enum) (.alignment (Variables|/Script/Wipgate.RTS_Entity|GetTeam _asrts_unit)) (Variables|Default|GetTargetAlignment))
    (bind _returnvalue (Class|GeneralFunctionLibraryCPP|CreateUnitEffect self (Variables|Default|GetEffectStat) (Variables|Default|GetEffectType) (Math|Float|Clamp(Float) (- _delay (Variables|Default|GetElapsed)) 0.0 _delay) (Variables|Default|GetMagnitude) (Variables|Default|GetDuration)))
    (Class|UnitEffect|SetParticles _returnvalue (Variables|Default|GetEffectParticle_Tick) (Variables|Default|GetEffectParticle_Start) (Variables|Default|GetEffectParticle_End) (Variables|Default|GetEffectParticle_Constant) (Variables|Default|GetSocketName))
    (Utilities|Map|Add (Variables|Default|GetUnitsAndEffects) _asrts_unit _returnvalue)
    (Class|RTSEntity|AddUnitEffect _asrts_unit _returnvalue)))

(event EventBeginPlay
  (bind _returnvalue (Components|GetOwner))
  ;[1 1 1] Set Height Offset
  (Utilities|IsValid _returnvalue
    (:Is%20Valid
      (bind _asrts_entity (Utilities|Casting|CastToRTS_Entity _returnvalue))
      (Variables|Default|SetHeightOffset (Components|Capsule|GetScaledCapsuleHalfHeight (Actor|GetComponentbyClass _asrts_entity "/Script/Engine.CapsuleComponent"))))))

(event EventTick
  (params (DeltaSeconds :type Float%20%28single-precision%29))
  ;[1 1 1] Destroy and remove effect after duration
  (CallFunction|UpdateLocation)
  (bind _output_get (Variables|Default|SetElapsed (+ (Variables|Default|GetElapsed) DeltaSeconds)))
  (if (>= _output_get (Math|Conversions|ToFloat(Integer) (+ (Variables|Default|GetDuration) (Math|Float|Truncate (Variables|Default|GetDelay)))))
    (bind _keys (Utilities|Map|Keys (Variables|Default|GetUnitsAndEffects)))
    (for _array_element _keys
      (Class|RTSEntity|RemoveUnitEffect _array_element (.Value (Utilities|Map|Find (Variables|Default|GetUnitsAndEffects) _array_element))))
    (Actor|DestroyActor)))

(fn ConstructionScript
  (bind _radius (Variables|Default|GetRadius))
  (Components|Sphere|SetSphereRadius (Variables|Default|GetSphereCollider) _radius true)
  (Transformation|SetRelativeScale3D (Variables|Default|GetPlane) (* (Math|Conversions|ToVector(Float) _radius) 0.02)))

(fn SetEffectParticles
  (params (Effect%20Tick :type Particle%20System%20Object%20Reference) (Effect%20Start :type Particle%20System%20Object%20Reference) (Effect%20End :type Particle%20System%20Object%20Reference) (Effect%20Constant :type Particle%20System%20Object%20Reference) (Socket%20Name :type Name))
  (bind _output_get (Variables|Default|SetEffectParticle_Tick Effect%20Tick))
  (bind _output_get_2 (Variables|Default|SetEffectParticle_Start Effect%20Start))
  (bind _output_get_3 (Variables|Default|SetEffectParticle_End Effect%20End))
  (bind _output_get_4 (Variables|Default|SetEffectParticle_Constant Effect%20Constant))
  (bind _output_get_5 (Variables|Default|SetSocketName Socket%20Name))
  ;[1 1 1] Add particles to already instantiated effects due to colision being faster than initialization
  (bind _keys (Utilities|Map|Keys (Variables|Default|GetUnitsAndEffects)))
  (for _array_element _keys
    (bind _values (Utilities|Map|Values (Variables|Default|GetUnitsAndEffects)))
    (for _array_element_2 _values
      (Class|UnitEffect|SetParticles _array_element_2 _output_get _output_get_2 _output_get_3 _output_get_4 _output_get_5)
      (Class|UnitEffect|StartParticleConstant _array_element_2 (Variables|Transformation|GetRootComponent)))))

(fn SetAreaParticles)

(fn UpdateLocation
  (bind _returnvalue (Components|GetOwner))
  (Utilities|IsValid _returnvalue
    (:Is%20Valid
      (Transformation|SetWorldLocation (Variables|Default|GetDefaultSceneRoot) (+ (Transformation|GetActorLocation _returnvalue) (Math|Vector|MakeVector 0.0 0.0 (- 25.0 (Variables|Default|GetHeightOffset)))) false false))))

(fn DestroyAreaOfEffect
  (bind _keys (Utilities|Map|Keys (Variables|Default|GetUnitsAndEffects)))
  (for _array_element _keys
    (Class|RTSEntity|RemoveUnitEffect _array_element (.Value (Utilities|Map|Find (Variables|Default|GetUnitsAndEffects) _array_element))))
  (Actor|DestroyActor))