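; Unit culling actor for the RTS camera, carrying a plane that is exposed through GetCullPlane.
; Each tick it billboards the plane toward the RTS camera pawn's camera.
; It then encodes the camera-to-cylinder distance, scaled down, in the red channel of the plane's vertex colours.
; The same distance becomes the plane's translucent sort priority, replacing the random one set at BeginPlay.
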(event EventBeginPlay
  (bind _asrts_camera_pawn (Utilities|Casting|CastToRTS_CameraPawn (Game|Player|GetPlayerPawn 0)))
  (Variables|Default|SetWorldCamera (Variables|/Game/Code/Blueprints/RTS_CameraPawn.RTS_CameraPawn_C|GetCamera _asrts_camera_pawn))
  (Rendering|SetTranslucentSortPriority (Variables|Default|GetPlane) (Math|Random|RandomInteger 50)))

(event Collision|EventActorBeginOverlap
  (params (OtherActor :type Actor%20Object%20Reference)))

(event EventTick
  (params (DeltaSeconds :type Float%20%28single-precision%29))
  (CallFunction|FacCamera)
  (CallFunction|Paint))

(fn ConstructionScript)

(fn FacCamera
  (bind _plane (Variables|Default|GetPlane))
  (Transformation|SetWorldRotation _plane (Math|Conversions|RotationFromXVector (Math|Vector|RotateVector (Math|Vector|Normalize (- (Transformation|GetWorldLocation (Variables|Default|GetWorldCamera)) (Transformation|GetWorldLocation (Variables|Default|GetPlane)))) "0, 0, 0")) false false)
  (Transformation|AddLocalRotation _plane "-90.000000,0.000000,0.000000" false false))

(fn Paint
  (bind _cylinder (Variables|Default|GetCylinder))
  (bind _worldcamera (Variables|Default|GetWorldCamera))
  (bind _returnvalue (Transformation|GetWorldLocation _worldcamera))
  (bind _returnvalue_2 (Transformation|GetWorldLocation _cylinder))
  (bind _returnvalue_3 (- _returnvalue _returnvalue_2))
  (bind _returnvalue_4 (Math|Vector|VectorLength _returnvalue_3))
  (bind _coloroutput (CallFunction|DistancetoColor _returnvalue_4))
  (Rendering|SetTranslucentSortPriority (Variables|Default|GetPlane) (Math|Float|Truncate _returnvalue_4))
  (Class|MeshVertexPainterKismetLibrary|PaintVerticesSingleColor (Variables|Default|GetPlane) _coloroutput false))

(fn DistancetoColor
  (params (Distance :type Float%20%28single-precision%29))
  (return (Utilities|Struct|MakeLinearColor (/ Distance 1e+04) 0.0 0.0 1.0)))

(fn GetCullPlane
  (return (Variables|Default|GetPlane)))