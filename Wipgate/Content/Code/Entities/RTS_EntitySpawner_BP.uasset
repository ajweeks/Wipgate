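; RTS entity spawner that, on SpawnEntities, places a set piece at its transform and populates the surrounding area with team-aligned entities.
; Each EntitySpawns entry spawns its amount of units at random navigable points within Radius, retrying up to SpawnAttempts per unit.
; Spawned units receive the spawner's Alignment through InitializeEntity, the set piece is initialized with the spawner, and failures print debug warnings.
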(event EventSpawnEntities
  (bind _returnvalue (Transformation|GetActorLocation))
  (bind _self self)
  (bind _radius (Variables|Default|GetRadius))
  (bind _setpiece (Variables|Default|GetSetPiece))
  (bind _returnvalue_2 (Utilities|GetObjectName _self))
  (bind (_randomlocation _returnvalue_3) (Class|NavigationSystem|GetRandomPointinNavigableRadius _returnvalue _radius))
  (bind _returnvalue_4 (Utilities|String|Append _returnvalue_2 " > " "Cannot spawn units in the specified radius"))
  (Variables|Default|Setm_IsActive true)
  (bind _returnvalue_5 (Game|SpawnActorfromClass _setpiece (Transformation|GetActorTransform) "Undefined" 0 0))
  (Utilities|IsValid _returnvalue_5
    (:Is%20Valid
      (Class|RTSSetPiece|Initialize _returnvalue_5 self))
    (:Is%20Not%20Valid
      (if (!= _setpiece 0)
        (Development|PrintString (Utilities|String|Append (Utilities|GetObjectName self) " > " "Cannot spawn set piece")))))
  (for _array_element (Variables|Default|GetEntitySpawns)
    (for _index (range 1 (.amount _array_element))
      (if _returnvalue_3
        (Variables|Default|SetObjectHasSpawned false)
        (Variables|Default|SetWhileIndex 0)
        (while (and (< (Variables|Default|GetWhileIndex) (Variables|Default|GetSpawnAttempts)) (not (Variables|Default|GetObjectHasSpawned)))
          (bind _returnvalue_6 (Game|SpawnActorfromClass (.entity _array_element) (Math|Conversions|ToTransform(Vector) _randomlocation) "Undefined" 0 0))
          (Utilities|IsValid _returnvalue_6
            (:Is%20Valid
              (Variables|Default|SetObjectHasSpawned true)
              (Variables|Default|SetWhileIndex (Variables|Default|GetSpawnAttempts))
              (Class|RTSEntitySpawner|InitializeEntity _returnvalue_6 (Variables|Default|GetAlignment)))
            (:Is%20Not%20Valid
              (Math|Integer|IncrementInt (Variables|Default|GetWhileIndex)))))
        (if (not (Variables|Default|GetObjectHasSpawned))
          (Development|PrintString _returnvalue_4))
        (else
          (Development|PrintString _returnvalue_4))))))

(fn ConstructionScript)