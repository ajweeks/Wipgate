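; RTS player spawn point that recreates the player's saved units around its location.
; SpawnEntities copies SavedEntities from the game instance, then spawns each entity at a random navigable point within Radius.
; Valid spawns are initialized on the player team and get their saved health and Luma stats back.
; Failed spawns loop back for retries bounded by SpawnAttempts, and a failed navigable-point lookup prints an error.
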(event EventSpawnEntities
  (bind _returnvalue (Transformation|GetActorLocation))
  (bind _radius (Variables|Default|GetRadius))
  (bind (_randomlocation _returnvalue_2) (Class|NavigationSystem|GetRandomPointinNavigableRadius _returnvalue _radius))
  (CallFunction|SetFriendlyUnits)
  (Variables|Default|Setm_IsActive true)
  (for _array_element (Variables|Default|GetSavedEntities)
    (if _returnvalue_2
      (bind _returnvalue_3 (Game|SpawnActorfromClass (.entity _array_element) (Math|Conversions|ToTransform(Vector) _randomlocation) "Undefined" 0 0 :!label _label))
      (Utilities|IsValid _returnvalue_3
        (:Is%20Valid
          (Variables|Default|SetObjectHasSpawned true)
          (Variables|Default|SetWhileIndex (Variables|Default|GetSpawnAttempts))
          (Class|RTSEntitySpawnerBase|InitializeEntity _returnvalue_3 "E_PLAYER")
          (Variables|/Script/Wipgate.RTS_Entity|SetHealth _returnvalue_3 (.health _array_element))
          (Variables|/Script/Wipgate.RTS_Entity|SetCurrentLumaStats _returnvalue_3 (.lumastats _array_element)))
        (:Is%20Not%20Valid
          (Variables|Default|SetObjectHasSpawned false)
          (Variables|Default|SetWhileIndex 0)
          (while (and (< (Variables|Default|GetWhileIndex) (Variables|Default|GetSpawnAttempts)) (not (Variables|Default|GetObjectHasSpawned)))
            (Math|Integer|IncrementInt (Variables|Default|GetWhileIndex)
              (:%20%20
                (goto _label))))
          (if (and (< (Variables|Default|GetWhileIndex) (Variables|Default|GetSpawnAttempts)) (not (Variables|Default|GetObjectHasSpawned)))
            (Development|PrintString (Utilities|String|Append (Utilities|GetObjectName self) " > " "Cannot spawn units in the specified radius") :!label _label_2))))
      (else
        (goto _label_2)))))

(fn ConstructionScript)

(fn SetFriendlyUnits
  (bind _asrts_game_instance_bp (Utilities|Casting|CastToRTS_GameInstance_BP (Game|GetGameInstance)))
  (Variables|Default|SetSavedEntities (Variables|/Script/Wipgate.RTS_GameInstance|GetSavedEntities _asrts_game_instance_bp)))