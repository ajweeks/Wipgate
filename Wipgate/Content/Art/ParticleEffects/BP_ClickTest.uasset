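; BP_ClickTest is a test actor that repeatedly spawns BP_ClickEffect around itself.
; On Tick it accumulates delta time and, each time the timer passes half a second, resets it and spawns the effect.
; Each spawn lands at a random point in a flat box centred on the actor and receives the actor's Color variable.
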(event EventBeginPlay)

(event Collision|EventActorBeginOverlap
  (params (OtherActor :type Actor%20Object%20Reference)))

(event EventTick
  (params (DeltaSeconds :type Float%20%28single-precision%29))
  (bind _output_get (Variables|Default|SetTimer (+ (Variables|Default|GetTimer) (Utilities|Time|GetWorldDeltaSeconds))))
  (Math|Float|CompareFloat _output_get 0.5
    (:>
      (Variables|Default|SetTimer 0.0)
      (Game|SpawnActorfromClass "/Game/Art/ParticleEffects/BP_ClickEffect.BP_ClickEffect_C" (Math|Transform|MakeTransform (Math|Random|RandomPointinBoundingBox (Transformation|GetActorLocation) (Math|Vector|MakeVector 1e+02 1e+02 0.0))) "Undefined" 0 (Variables|Default|GetColor) 0))))

(fn ConstructionScript)