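; BP_AOE_Effect is a configurable area-of-effect skill visual made of an icon plane and a range cylinder.
; The construction script scales the cylinder from Radius and RangeHeight, leaving the plane's scale untouched.
; It creates dynamic instances of M_AOEPlane and M_AOERange, feeding Color and Icon to the plane and a brightened Color to the cylinder.
; All setup happens at construction, with no active runtime logic.
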(event EventBeginPlay)

(event Collision|EventActorBeginOverlap
  (params (OtherActor :type Actor%20Object%20Reference)))

(event EventTick
  (params (DeltaSeconds :type Float%20%28single-precision%29)))

(fn ConstructionScript
  (bind _radius (Variables|Default|GetRadius))
  (bind _returnvalue (/ _radius 5e+01))
  (Transformation|SetRelativeScale3D (Variables|Default|GetRangeCylinder) (Math|Vector|MakeVector _returnvalue _returnvalue (/ (Variables|Default|GetRangeHeight) 1e+02)))
  (bind _returnvalue_2 (Rendering|Material|CreateDynamicMaterialInstance "/Game/Art/ParticleEffects/AOESkills/M_AOEPlane.M_AOEPlane" :!class /Script/Engine.KismetMaterialLibrary))
  (bind _output_get (LocalVariables|SetplaneMaterial _returnvalue_2))
  (Rendering|Material|SetVectorParameterValue _output_get "Color" (Variables|Default|GetColor) :!class /Script/Engine.MaterialInstanceDynamic)
  (Rendering|Material|SetTextureParameterValue (LocalVariables|GetplaneMaterial) "Icon" (Variables|Default|GetIcon))
  (bind _returnvalue_3 (Rendering|Material|CreateDynamicMaterialInstance "/Game/Art/ParticleEffects/AOESkills/M_AOERange.M_AOERange" :!class /Script/Engine.KismetMaterialLibrary))
  (bind _output_get_2 (LocalVariables|SetrangeMaterial _returnvalue_3))
  (Rendering|Material|SetVectorParameterValue _output_get_2 "Color" (* (Variables|Default|GetColor) 5.0) :!class /Script/Engine.MaterialInstanceDynamic)
  (Rendering|Material|SetMaterial (Variables|Default|GetEffectPlane) 0 (LocalVariables|GetplaneMaterial))
  (Rendering|Material|SetMaterial (Variables|Default|GetRangeCylinder) 0 (LocalVariables|GetrangeMaterial)))