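; BP_ClickEffect is a short-lived ground click effect actor drawn on a plane.
; The construction script gives the plane a dynamic instance of the ground click material and applies the Color variable to it.
; Tick advances a timer scaled by Speed, feeds it to the material's Time parameter to drive the animation, and destroys the actor once the timer exceeds one.
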(event EventBeginPlay)

(event Collision|EventActorBeginOverlap
  (params (OtherActor :type Actor%20Object%20Reference)))

(event EventTick
  (params (DeltaSeconds :type Float%20%28single-precision%29))
  (Variables|Default|SetTimer (+ (Variables|Default|GetTimer) (* (Utilities|Time|GetWorldDeltaSeconds) (Variables|Default|GetSpeed))))
  (Rendering|Material|SetScalarParameterValue (Variables|Default|GetMatInstance) "Time" (Variables|Default|GetTimer) :!class /Script/Engine.MaterialInstanceDynamic)
  (Math|Float|CompareFloat (Variables|Default|GetTimer) 1.0
    (:>
      (Actor|DestroyActor))))

(fn ConstructionScript
  (bind _returnvalue (Rendering|Material|CreateDynamicMaterialInstance (Variables|Default|GetPlane) 0 "/Game/Art/ParticleEffects/ClickEffect/PE_M_GroundClick_Inst.PE_M_GroundClick_Inst" :!class /Script/Engine.PrimitiveComponent))
  (bind _output_get (Variables|Default|SetMatInstance _returnvalue))
  (Rendering|Material|SetMaterial (Variables|Default|GetPlane) 0 _output_get)
  (Rendering|Material|SetVectorParameterValueonMaterials (Variables|Default|GetPlane) "Color" (Math|Conversions|ToVector(LinearColor) (Variables|Default|GetColor))))