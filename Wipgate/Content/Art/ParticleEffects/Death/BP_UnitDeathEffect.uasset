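; BP_UnitDeathEffect is a unit death effect actor that shows a blood decal and a currency gain widget.
; On BeginPlay it applies a dynamic blood decal material and starts the RTS_CurrencyGain widget animation with the effect lifetime.
; Tick ramps the decal's BloodAmountScale to full shortly after spawn.
; WidgetTick, which lifts the widget with decaying speed and destroys it after that lifetime, is disconnected as work in progress.
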(event EventBeginPlay
  (bind _returnvalue (Rendering|Material|CreateDynamicMaterialInstance "/Game/Art/ParticleEffects/Death/M_BloodDecal_Inst.M_BloodDecal_Inst" :!class /Script/Engine.KismetMaterialLibrary))
  (bind _output_get (Variables|Default|SetDecalMatInstance _returnvalue))
  (Rendering|Components|Decal|SetDecalMaterial (Variables|Default|GetDecal) _output_get)
  (bind _asrts_currency_gain (Utilities|Casting|CastToRTS_CurrencyGain (UserInterface|GetUserWidgetObject (Variables|Default|GetWidget))))
  (Default|StartAnim _asrts_currency_gain (Variables|Default|GetCurrency%20Effect%20Lifetime)))

(event Collision|EventActorBeginOverlap
  (params (OtherActor :type Actor%20Object%20Reference)))

(event EventTick
  (params (DeltaSeconds :type Float%20%28single-precision%29))
  (Rendering|Material|SetScalarParameterValue (Variables|Default|GetDecalMatInstance) "BloodAmountScale" (Math|Float|Clamp(Float) (Math|Float|Power (/ (Actor|GetGameTimeSinceCreation) 0.2) 1.0)) :!class /Script/Engine.MaterialInstanceDynamic))

(fn ConstructionScript)